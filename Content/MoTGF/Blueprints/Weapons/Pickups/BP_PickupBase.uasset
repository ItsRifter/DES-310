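; Base actor for weapon pickups that hands a given weapon to the player.
; Its Pickup event sets the weapon as the player's active weapon and adds it to their inventory for immediate use.
; It also stores the weapon class in the game instance as the carried weapon, then destroys every pickup actor in the world, so taking one removes all the others.
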(event `Pickup`
  (params (WeaponBase :type "/Game/MoTGF/Blueprints/Weapons/BP_WeaponBase Object Reference"))
  (bind _asbp_player (cast `/Game/MoTGF/Blueprints/Player/BP_Player` (`GameplayStatics.GetPlayerCharacter` 0)))
  (set `/Game/MoTGF/Blueprints/Player/BP_Player.ActiveWeapon` WeaponBase _asbp_player)
  (`/Game/MoTGF/Blueprints/Player/BP_Inventory.AddWeapon` (`/Game/MoTGF/Blueprints/Player/BP_Player.Inventory` _asbp_player) true WeaponBase)
  (bind _asbp_mo_tgf_game_instance (cast `/Game/MoTGF/Blueprints/Gameplay/BP_MoTGF_GameInstance` (`GameplayStatics.GetGameInstance`)))
  (set `/Game/MoTGF/Blueprints/Gameplay/BP_MoTGF_GameInstance.CarryingWeapon` (`GameplayStatics.GetObjectClass` WeaponBase) _asbp_mo_tgf_game_instance)
  (bind _outactors (`GameplayStatics.GetAllActorsOfClass` "BP_PickupBase_C"))
  (for _array_element _outactors
    (`self.K2_DestroyActor` _array_element)))

(fn `UserConstructionScript`)