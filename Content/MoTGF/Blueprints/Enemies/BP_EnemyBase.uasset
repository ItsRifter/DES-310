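; Base enemy character that handles health, hit reactions, death and attack hooks for child enemies.
; Damage plays a sound matching the player's weapon, updates the health widget, triggers Niagara VFX and launches knockable enemies away, scaled by weapon knockback.
; Death notifies MoTGF_GameState and drops a random item when a roll meets or exceeds ItemDropChance.
; Tick calls the empty TryDoAttacks hook while alive, and helpers set AI blackboard attack and charge flags.
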(event `OnDamaged`
  (params (Damage :type Integer))
  (bind _asbp_player (cast `/Game/MoTGF/Blueprints/Player/BP_Player` (`GameplayStatics.GetPlayerCharacter` 0)))
  (bind _returnvalue (`GameplayStatics.GetObjectClass` (`/Game/MoTGF/Blueprints/Player/BP_Player.ActiveWeapon` _asbp_player)))
  (if (== _returnvalue "/Game/MoTGF/Blueprints/Weapons/Weapons/Scythe/BP_Wep_Scythe.BP_Wep_Scythe_C")
    (`GameplayStatics.PlaySoundAtLocation` "/Game/MoTGF/Sounds/Weapons/scythe_slash.scythe_slash" (`self.K2_GetActorLocation`) (struct) 1.0 1.0 0.0 null null null null)
    (elif (== _returnvalue "/Game/MoTGF/Blueprints/Weapons/Weapons/Pitchfork/Bp_Wep_Pitchfork.Bp_Wep_Pitchfork_C")
      (`GameplayStatics.PlaySoundAtLocation` "/Game/MoTGF/Sounds/Weapons/pitchfork_stab.pitchfork_stab" (`self.K2_GetActorLocation`) (struct) 1.0 1.0 0.0 null null null null)
      (else
        (`GameplayStatics.PlaySoundAtLocation` "/Game/MoTGF/Sounds/Weapons/shovel_hit.shovel_hit" (`self.K2_GetActorLocation`) (struct) 1.0 1.0 0.0 null null null null))))
  (bind _output_get (set `self.CurrentHealth` (- (`self.CurrentHealth`) Damage)))
  (`/Game/MoTGF/Blueprints/UI/BP_EnemyHealthUI.Update Health` (`self.HealthUI`) _output_get)
  (`self.DoKnockback`)
  (if (<= (`self.CurrentHealth`) 0)
    (`ActorComponent.Activate` (`self.NiagaraVFX`) true)
    (`self.OnDeath`)
    (else
      (`ActorComponent.Activate` (`self.NiagaraVFX`) true))))

(event `self.ReceiveBeginPlay`
  (`self.DoPlaySound` (`self.AlertSound`))
  (bind _asbp_enemy_health_ui (cast `/Game/MoTGF/Blueprints/UI/BP_EnemyHealthUI` (`WidgetComponent.GetUserWidgetObject` (`self.Health`))))
  (set `self.HealthUI` _asbp_enemy_health_ui)
  (bind _output_get (set `self.CurrentHealth` (`self.MaxHealth`)))
  (set `/Game/MoTGF/Blueprints/UI/BP_EnemyHealthUI.CurrentHealth` _output_get (`self.HealthUI`))
  (set `/Game/MoTGF/Blueprints/UI/BP_EnemyHealthUI.MaxHealth` (`self.MaxHealth`) (`self.HealthUI`))
  (set `/Game/MoTGF/Blueprints/UI/BP_EnemyHealthUI.Enemy Type` (`self.EnemyName`) (`self.HealthUI`))
  (`/Game/MoTGF/Blueprints/UI/BP_EnemyHealthUI.Update Health` (`self.HealthUI`) (`self.CurrentHealth`))
  (`self.SpawnDefaultController`))

(event `self.ReceiveAnyDamage`
  (params (Damage :type "Float (single-precision)") (DamageType :type "DamageType Object Reference") (InstigatedBy :type "Controller Object Reference") (DamageCauser :type "Actor Object Reference"))
  (`self.OnDamaged` (`KismetMathLibrary.Round` Damage)))

(event `OnDeath`
  (bind _mesh (`self.Mesh`))
  (set `self.IsDead` true)
  (if (>= (`KismetMathLibrary.RandomIntegerInRange` 0 100) (`self.ItemDropChance`))
    (`|SpawnActorFromClass` (`KismetArrayLibrary.Array_Random` (`self.ItemDrops`)) (`KismetMathLibrary.MakeTransform` (`self.K2_GetActorLocation` self)) "Undefined" "MultiplyWithRoot" null null)
    (bind _asmo_tgf_game_state (cast `/Game/MoTGF/Blueprints/Gameplay/MoTGF_GameState` (`GameplayStatics.GetGameState`)))
    (`/Game/MoTGF/Blueprints/Gameplay/MoTGF_GameState.EnemyDeath` _asmo_tgf_game_state)
    (`PrimitiveComponent.SetCollisionEnabled` _mesh "NoCollision")
    (`SceneComponent.SetVisibility` _mesh false false)
    (`self.K2_DestroyActor`)
    (else
      (bind _asmo_tgf_game_state_2 (cast `/Game/MoTGF/Blueprints/Gameplay/MoTGF_GameState` (`GameplayStatics.GetGameState`)))
      (`/Game/MoTGF/Blueprints/Gameplay/MoTGF_GameState.EnemyDeath` _asmo_tgf_game_state_2)
      (`self.K2_DestroyActor`))))

(event `DoChargingAttack`
  (bind _output_get (set `self.IsAttackCharging` true))
  (`BlackboardComponent.SetValueAsBool` (`AIBlueprintHelperLibrary.GetBlackboard` (`AIBlueprintHelperLibrary.GetAIController` self)) "IsCharging" _output_get))

(event `StopChargeAttack`
  (bind _output_get (set `self.IsAttackCharging` false))
  (`BlackboardComponent.SetValueAsBool` (`AIBlueprintHelperLibrary.GetBlackboard` (`AIBlueprintHelperLibrary.GetAIController` self)) "IsCharging" _output_get)
  (`self.FinishAttack`))

(event `DoAttack`)

(event `TryDoAttacks`)

(event `StartAttack`)

(event `FinishAttack`
  (`self.SetAttackValue` false))

(event `self.ReceiveTick`
  (params (DeltaSeconds :type "Float (single-precision)"))
  (if (not (`self.IsDead`))
    (`self.TryDoAttacks`)))

(event `Ready`)

(event `DoKnockback`
  (if (`self.IsKnockable`)
    (bind _asbp_player (cast `/Game/MoTGF/Blueprints/Player/BP_Player` (`GameplayStatics.GetPlayerCharacter` 0)))
    (`MovementComponent.StopMovementImmediately` (`self.CharacterMovement`))
    (bind _asbp_player_2 (cast `/Game/MoTGF/Blueprints/Player/BP_Player` (`GameplayStatics.GetPlayerCharacter` 0)))
    (bind (_returnvalue_x _returnvalue_y _returnvalue_z) (`KismetMathLibrary.BreakVector` (`KismetMathLibrary.GetDirectionUnitVector` (`SceneComponent.K2_GetComponentLocation` (`Character.CapsuleComponent` _asbp_player_2)) (`self.K2_GetActorLocation`))))
    (`self.LaunchCharacter` (* (`KismetMathLibrary.MakeVector` _returnvalue_x _returnvalue_y (+ _returnvalue_z 1.0)) (`/Game/MoTGF/Blueprints/Weapons/BP_WeaponBase.Knockback` (`/Game/MoTGF/Blueprints/Player/BP_Player.ActiveWeapon` _asbp_player))))))

(event `DestroyWidget`
  (`ActorComponent.K2_DestroyComponent` (`self.Health`)))

(fn `CanDoAttack`
  (returns (Result :type Boolean))
  (return (<= (`KismetMathLibrary.Vector_Distance` (`self.K2_GetActorLocation`) (`self.K2_GetActorLocation` (`GameplayStatics.GetPlayerPawn` 0))) (`self.AttackRange`))))

(fn `DoPlaySound`
  (params (Sound :type "SoundCue Object Reference") (Pitch :type "Float (double-precision)" :default 1.0))
  (bind _audioplayer (`self.AudioPlayer`))
  (`AudioComponent.SetPitchMultiplier` _audioplayer Pitch)
  (`AudioComponent.SetSound` _audioplayer Sound)
  (`AudioComponent.Play` _audioplayer 0.0))

(fn `GetVectorAngle`
  (params (VecA :type "Vector Structure") (VecB :type "Vector Structure"))
  (returns (Angle :type "Float (double-precision)"))
  (return (`KismetMathLibrary.DegAcos` (`KismetMathLibrary.Dot_VectorVector` (`KismetMathLibrary.Normal` VecA) (`KismetMathLibrary.Normal` VecB)))))

(fn `SetAttackValue`
  (params (Value :type Boolean))
  (bind _returnvalue (`AIBlueprintHelperLibrary.GetBlackboard` (`AIBlueprintHelperLibrary.GetAIController` self)))
  (if Value
    (`BlackboardComponent.SetValueAsBool` _returnvalue "CanAttackPlayer" true)
    (else
      (`BlackboardComponent.SetValueAsBool` _returnvalue "CanAttackPlayer" false))))

(fn `UserConstructionScript`)