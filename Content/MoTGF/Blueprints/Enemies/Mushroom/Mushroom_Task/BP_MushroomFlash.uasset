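; Behavior tree task that makes the mushroom enemy telegraph with a one-second warning, likely ahead of an attack.
; On execute it casts the pawn to BP_Mushroom, turns off the animation's bounce, shows the enemy warning component and plays the charge sound at the mushroom's location.
; After the delay it hides the warning and finishes successfully; a failed cast never calls FinishExecute.
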(event `self.ReceiveExecuteAI`
  (params (OwnerController :type "AIController Object Reference") (ControlledPawn :type "Pawn Object Reference"))
  (bind _asbp_mushroom (cast `/Game/MoTGF/Blueprints/Enemies/Mushroom/BP_Mushroom` ControlledPawn))
  (set `/Game/MoTGF/Animations/Shroom/MushroomAnimBlueprint.DoBounce` false (`/Game/MoTGF/Blueprints/Enemies/Mushroom/BP_Mushroom.Animation reference` _asbp_mushroom))
  (bind _enemywarning (`/Game/MoTGF/Blueprints/Enemies/Mushroom/BP_Mushroom.EnemyWarning` _asbp_mushroom))
  (`SceneComponent.SetVisibility` _enemywarning true false)
  (`GameplayStatics.PlaySoundAtLocation` (`/Game/MoTGF/Blueprints/Enemies/BP_EnemyBase.ChargeSound` _asbp_mushroom) (`Actor.K2_GetActorLocation` _asbp_mushroom) (struct) 1.0 1.0 0.0 null null null null)
  (`KismetSystemLibrary.Delay` 1.0)
  (`SceneComponent.SetVisibility` _enemywarning false false)
  (`self.FinishExecute` true))