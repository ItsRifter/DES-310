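; BP_Skill_Health is a player skill that raises the player's Health each time it is upgraded.
; Upgrade calls the parent, gets the player reference from player character 0, and adds HealthUpPerLevel to its Health with no clamp.
; It then prints the new value to screen as debug output.
; CreateSkill only passes the Player through to the parent implementation.
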(event `self.CreateSkill`
  (params (Player :type "/Game/David/Blueprints/Player/BP_Player Object Reference"))
  (`parent.CreateSkill` Player))

(event `self.Upgrade`
  (`parent.Upgrade`)
  (bind _playerref (`/Engine/EditorBlueprintResources/StandardMacros.GetPlayerRef` (`GameplayStatics.GetPlayerCharacter` 0))
    (:`Result`
      (bind _output_get (set `/Game/David/Blueprints/Player/BP_Player.Health` (+ (`self.HealthUpPerLevel`) (`/Game/David/Blueprints/Player/BP_Player.Health` _playerref)) _playerref))
      (`KismetSystemLibrary.PrintString` (`KismetStringLibrary.Conv_DoubleToString` _output_get)))))