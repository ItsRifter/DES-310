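; BP_Mushroom is an enemy that bounces until it attacks with a cloud, light and sound.
; Attack pauses the anim Blueprint's bounce and runs a single 150-unit sphere trace ignoring "Enemy"-tagged actors, damaging the player pawn on any hit.
; Ready stops the effects and resumes bouncing after a short delay.
; Both events call end notifications, while BeginPlay and damage also run parent logic.
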(event `self.ReceiveBeginPlay`
  (bind _asmushroom_anim_blueprint (cast `/Game/MoTGF/Animations/Shroom/MushroomAnimBlueprint` (`SkeletalMeshComponent.GetAnimInstance` (`self.Mesh`))))
  (set `self.Animation reference` _asmushroom_anim_blueprint)
  (set `/Game/MoTGF/Animations/Shroom/MushroomAnimBlueprint.DoBounce` true (`self.Animation reference`))
  (`ActorComponent.Deactivate` (`self.Cloud1`))
  (bind _asbp_enemy_health_ui (cast `/Game/MoTGF/Blueprints/UI/BP_EnemyHealthUI` (`WidgetComponent.GetUserWidgetObject` (`self.Health`))))
  (set `self.HealthUI` _asbp_enemy_health_ui)
  (`parent.ReceiveBeginPlay`))

(event `Attack`
  (bind _cloud1 (`self.Cloud1`))
  (bind _returnvalue (`self.K2_GetActorLocation` self))
  (bind _returnvalue_2 (`GameplayStatics.SpawnSoundAtLocation` (`self.AttackSound`) (`self.K2_GetActorLocation`) (struct) 1.0 1.0 0.0 null null))
  (set `self.ActiveAttackSound` _returnvalue_2)
  (set `/Game/MoTGF/Animations/Shroom/MushroomAnimBlueprint.DoBounce` false (`self.Animation reference`))
  (`SceneComponent.SetVisibility` (`self.PointLight`) true false)
  (`NiagaraComponent.SetVariablePosition` _cloud1 "None" (`self.K2_GetActorLocation` self))
  (`ActorComponent.Activate` _cloud1 false)
  (bind _outactors (`GameplayStatics.GetAllActorsWithTag` "Enemy"))
  (bind (_outhit _returnvalue_3) (`KismetSystemLibrary.SphereTraceSingleForObjects` _returnvalue _returnvalue 150.0 (`|MakeArray` "ObjectTypeQuery3" :!type "EObjectTypeQuery Enum") false _outactors "None" true (struct :`R` 1.0 :`A` 1.0) (struct :`G` 1.0 :`A` 1.0) (`self.CloudDuration`)))
  (if _returnvalue_3
    (bind _asbp_player (cast `/Game/MoTGF/Blueprints/Player/BP_Player` (`GameplayStatics.GetPlayerPawn` 0)))
    (`GameplayStatics.ApplyDamage` _asbp_player 1.0)
    (`GameplayStatics.PlaySound2D` (`self.HitSound`) 1.0 1.0 0.0 null null)
    (`self.OnAttackEnd`)
    (else
      (`self.OnAttackEnd`))))

(event `Ready`
  (`AudioComponent.Stop` (`self.ActiveAttackSound`))
  (`ActorComponent.Deactivate` (`self.Cloud1`))
  (`SceneComponent.SetVisibility` (`self.PointLight`) false false)
  (`self.OnReadyEnd`)
  (`KismetSystemLibrary.Delay` 0.2)
  (set `/Game/MoTGF/Animations/Shroom/MushroomAnimBlueprint.DoBounce` true (`self.Animation reference`)))

(event `self.ReceiveAnyDamage`
  (params (Damage :type "Float (single-precision)") (DamageType :type "DamageType Object Reference") (InstigatedBy :type "Controller Object Reference") (DamageCauser :type "Actor Object Reference"))
  (`parent.ReceiveAnyDamage` Damage null null null))

(fn `UserConstructionScript`)