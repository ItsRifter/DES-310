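; Base weapon actor for the player that attaches on obtain, shows only while in use, and offers attack methods for child weapons.
; Stab, stepped-arc box sweeps and radius sphere traces filter hits by exact class, apply damage and slow the player.
; The arc ignores already-hit targets between steps, and a projectile attack spawns a projectile initialized with the weapon.
; DoAttack starts a cooldown that counts down on Tick.
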(event `StartUsing`
  ;[1 1 1] Start/Stop using
  (`SceneComponent.SetVisibility` (`self.DefaultSceneRoot`) true true)
  (set `/Game/MoTGF/Blueprints/Player/BP_Player.ActiveWeapon` self (`self.Player`)))

(event `self.ReceiveBeginPlay`
  ;[1 1 1] Setup on BeginPlay
  (`SceneComponent.SetVisibility` (`self.DefaultSceneRoot`) false true)
  (bind _asbp_player (cast `/Game/MoTGF/Blueprints/Player/BP_Player` (`GameplayStatics.GetPlayerCharacter` 0)))
  (set `self.playerRef` _asbp_player))

(event `StopUsing`
  ;[1 1 1] Start/Stop using
  (`SceneComponent.SetVisibility` (`self.DefaultSceneRoot`) false true))

(event `OnObtain`
  (params (Player :type "/Game/MoTGF/Blueprints/Player/BP_Player Object Reference"))
  (bind _holder (`/Game/MoTGF/Blueprints/Player/BP_Player.Holder` (`self.Player`)))
  ;[1 1 1] On obtaining this item
  (bind _output_get (set `self.Player` Player))
  (`self.K2_AttachToActor` _output_get "head" "KeepRelative" "KeepRelative" "KeepRelative" false)
  (`self.K2_SetActorLocationAndRotation` (`SceneComponent.K2_GetComponentLocation` _holder) (`SceneComponent.K2_GetComponentRotation` _holder)))

(event `DoStabAttack`
  (bind _returnvalue (`GameplayStatics.GetPlayerCharacter` 0))
  (bind _returnvalue_2 (`self.K2_GetActorLocation` _returnvalue))
  (bind _returnvalue_3 (`self.GetActorForwardVector` _returnvalue))
  (bind (_returnvalue_roll _returnvalue_pitch _returnvalue_yaw) (`KismetMathLibrary.BreakRotator` (`KismetMathLibrary.Conv_VectorToRotator` _returnvalue_3)))
  ;[1 1 1] Attack Methods
  ;;[0 0.2129 1] Stab Attack
  (bind _outhits (`KismetSystemLibrary.BoxTraceMultiForObjects` _returnvalue_2 (+ _returnvalue_2 (* _returnvalue_3 (`self.Range`))) (`self.StabHalfBoxScale`) (`KismetMathLibrary.MakeRotator` 0.0 0.0 _returnvalue_yaw) (`|MakeArray` "ObjectTypeQuery2" :!type "EObjectTypeQuery Enum") false (`|MakeArray` (`GameplayStatics.GetPlayerCharacter` 0) :!type "Actor Object Reference") "ForDuration" true (struct :`G` 0.946757 :`B` 1.0 :`A` 1.0)))
  (`self.CollectHitTargets` _outhits)
  (`self.DoDamage`)
  (`/Game/MoTGF/Blueprints/Player/BP_Player.WeaponSlow` (`self.playerRef`) (`self.Slow Ammount`)))

(event `DoArcAttack`
  (bind _returnvalue (`GameplayStatics.GetPlayerCharacter` 0))
  (bind _returnvalue_2 (`self.K2_GetActorLocation` _returnvalue))
  ;[1 1 1] Attack Methods
  ;;[0 0.85 1] Arc / Swing Attack - Shovel
  (`KismetArrayLibrary.Array_Add` (`self.IgnoreActors`) (`GameplayStatics.GetPlayerPawn` 0))
  (for _index (range 1 (+ (`self.Steps`) 1))
    (set `self.ArcIndex` _index)
    (bind _outhits (`KismetSystemLibrary.BoxTraceMultiForObjects` _returnvalue_2 (+ _returnvalue_2 (* (`KismetMathLibrary.GreaterGreater_VectorRotator` (`self.GetActorForwardVector` _returnvalue) (`KismetMathLibrary.MakeRotator` 0.0 0.0 (+ (* (`self.ArcDistance`) -0.5) (* (/ (`self.ArcDistance`) (`self.Steps`)) (`self.ArcIndex`))))) (`self.Range`))) (`self.ArcHalfBoxScale`) (struct) (`|MakeArray` "ObjectTypeQuery2" :!type "EObjectTypeQuery Enum") false (`self.IgnoreActors`) "ForDuration" true (struct :`G` 0.959756 :`B` 1.0 :`A` 1.0)))
    (`self.CollectHitTargets` _outhits)
    (`/Game/MoTGF/Blueprints/Player/BP_Player.WeaponSlow` (`self.playerRef`) (`self.Slow Ammount`)))
  (`self.DoDamage`)
  (`KismetArrayLibrary.Array_Clear` (`self.IgnoreActors`)))

(event `DoAttack`
  ;[1 1 1] Do attacking from input - each child weapon will use their specific attack method
  (bind _canattack_ (`self.CanAttack`))
  (if _canattack_
    (set `self.CurCooldown` (`self.Cooldown`))))

(event `DoRadiusAttack`
  (bind _array (`|MakeArray` "ObjectTypeQuery2" :!type "EObjectTypeQuery Enum"))
  (bind _radius (`self.Radius`))
  (bind _position (`self.Position`))
  (bind _array_2 (`|MakeArray` (`GameplayStatics.GetPlayerCharacter` 0) :!type "Actor Object Reference"))
  (bind _returnvalue (+ (* (`KismetMathLibrary.Vector_Down`) 32.0) (`self.K2_GetActorLocation` (`GameplayStatics.GetPlayerCharacter` 0))))
  ;[1 1 1] Attack Methods
  ;;[0.4838 1 0] Circle / Radius Attack - Scythe
  (if (`KismetMathLibrary.Vector_IsZero` (`self.Position`))
    (bind _outhits (`KismetSystemLibrary.SphereTraceMultiForObjects` _returnvalue _returnvalue _radius _array false _array_2 "ForDuration" true (struct :`R` 1.0 :`A` 1.0) (struct :`G` 1.0 :`A` 1.0) 3.0))
    (`self.CollectHitTargets` _outhits)
    (else
      (bind _outhits_2 (`KismetSystemLibrary.SphereTraceMultiForObjects` _position _position _radius _array false _array_2 "ForDuration" true (struct :`R` 1.0 :`A` 1.0) (struct :`G` 1.0 :`A` 1.0) 3.0))
      (`self.CollectHitTargets` _outhits_2)))
  (`self.DoDamage`)
  (`/Game/MoTGF/Blueprints/Player/BP_Player.WeaponSlow` (`self.playerRef`) (`self.Slow Ammount`)))

(event `DoDamage`
  ;[1 1 1] Attack Handling
  ;;[1 0.0414 0] Applies the damage and starts cooldown
  (if (`KismetArrayLibrary.Array_IsNotEmpty` (`self.HitTargets`))
    (for _array_element (`self.HitTargets`)
      (`GameplayStatics.ApplyDamage` _array_element (`self.Damage`) (`GameplayStatics.GetPlayerController` 0)))
    (`KismetArrayLibrary.Array_Clear` (`self.HitTargets`))))

(event `IncreaseDamage`
  (set `self.Damage` (+ (`self.Damage`) 1.0)))

(event `DoProjectileAttack`
  (bind _returnvalue (`GameplayStatics.GetPlayerPawn` 0))
  (bind _returnvalue_2 (`self.K2_GetActorRotation` _returnvalue))
  ;[1 1 1] Attack Methods
  ;;[0 1 0.03886] Projectile Attack
  (bind _returnvalue_3 (`|SpawnActorFromClass` (`self.Projectile`) (`KismetMathLibrary.MakeTransform` (+ (+ (* (`KismetMathLibrary.Vector_Up`) 48.0) (`self.K2_GetActorLocation` _returnvalue)) (* (`KismetMathLibrary.GetForwardVector` _returnvalue_2) 32.0)) _returnvalue_2) "AlwaysSpawn" "MultiplyWithRoot" null _returnvalue))
  (`/Game/MoTGF/Blueprints/Weapons/BP_ProjectileBase.SetupProjectile` _returnvalue_3 self))

(event `CollectHitTargets`
  (params (HitResults :type "Array of HitResult Structure"))
  ;[1 1 1] Attack Handling
  ;;[0 0.9598 1] Collects all hit targets from an attack separating unnecessary actors
  (for _array_element HitResults
    (bind (_bblockinghit _binitialoverlap _time _distance _location _impactpoint _normal _impactnormal _physmat _hitactor) (`GameplayStatics.BreakHitResult` _array_element))
    (bind _isvalidtype (`self.IsValidTargetType` _hitactor))
    (if _isvalidtype
      (`KismetArrayLibrary.Array_Add` (`self.HitTargets`) _hitactor)
      (`KismetArrayLibrary.Array_Add` (`self.IgnoreActors`) _hitactor))))

(event `ApplyCooldown`
  ;[1 1 1] Attack Handling
  (set `self.CurCooldown` (`self.Cooldown`)))

(event `self.ReceiveTick`
  (params (DeltaSeconds :type "Float (single-precision)"))
  ;[1 1 1] Attack Handling
  (if (> (`self.CurCooldown`) 0.0)
    (set `self.CurCooldown` (- (`self.CurCooldown`) (* DeltaSeconds 1.0)))))

(fn `CanAttack`
  (returns (`CanAttack?` :type Boolean))
  (return (<= (`self.CurCooldown`) 0.0)))

(fn `IsValidTargetType`
  (params (Target :type "Actor Object Reference"))
  (returns (IsValidType :type Boolean))
  (for _array_element (`self.ValidTypes`)
    (if (== (`GameplayStatics.GetObjectClass` Target) _array_element)
      (return true) ; A type matched, return true
    ))
  (return false) ; Types did not match actor, return false
)

(fn `UserConstructionScript`)