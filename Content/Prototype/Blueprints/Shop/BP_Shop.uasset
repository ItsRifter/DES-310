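; BP_Shop is a prototype shop actor that picks a random stock of items from a pool of possible item classes.
; ShuffleItems loops until it gathers three unique valid classes or reaches an attempt limit, then copies them to BuyableItems and clears the working list.
; Debug prints report additions and failed searches.
; Open, close and BeginPlay events are empty, and the only call to ShuffleItems is disconnected.
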(event `self.ReceiveBeginPlay`)

(event `OpenShop`)

(event `CloseShop`)

(event `ShuffleItems`
  (bind _itemstoadd (`self.ItemsToAdd`))
  ;[1 1 1] Shuffle items
  (while (not (or (>= (`KismetArrayLibrary.Array_Length` (`self.ItemsToAdd`)) 3) (>= (`self.ItemAttempts`) (`self.MaxAttempts`))))
    (bind _item (`self.GetRandomItem`))
    (if (`KismetSystemLibrary.IsValidClass` _item)
      (bind _isinstock (`self.HasItemForAdding` _item))
      (if _isinstock
        (`/Engine/EditorBlueprintResources/StandardMacros.IncrementInt` (`self.ItemAttempts`))
        (else
          (`KismetArrayLibrary.Array_Add` (`self.ItemsToAdd`) _item)
          (set `self.HasItemAdded` true)
          (set `self.ItemAttempts` 0)
          (`KismetSystemLibrary.PrintString` (`KismetStringLibrary.Concat_StrStr` (`KismetSystemLibrary.GetClassDisplayName` _item) " was added to the shop") true true (struct :`G` 0.66 :`B` 1.0 :`A` 1.0) 2.5)))
      (else
        (`/Engine/EditorBlueprintResources/StandardMacros.IncrementInt` (`self.ItemAttempts`)))))
  (set `self.BuyableItems` _itemstoadd)
  (`KismetArrayLibrary.Array_Clear` _itemstoadd)
  (if (>= (`self.ItemAttempts`) (`self.MaxAttempts`))
    (`KismetSystemLibrary.PrintString` "Too many attempts were made in getting items"))
  (set `self.ItemAttempts` 0))

(fn `GetRandomItem`
  (returns (Item :type "Actor Class Reference"))
  (return (`|GetArrayItem` (`self.PossibleItems`) (`KismetMathLibrary.RandomIntegerInRange` 0 (`KismetArrayLibrary.Array_Length` (`self.PossibleItems`))))))

(fn `HasItemForAdding`
  (params (Item :type "Actor Class Reference"))
  (returns (IsInStock :type Boolean))
  (return (!= (`KismetArrayLibrary.Array_Find` (`self.ItemsToAdd`) Item) -1)))

(fn `UserConstructionScript`)