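; BP_Coins is a spinning coin pickup that adds its Value to the player's pending money on overlap, then plays a sound and destroys itself.
; The construction script compares Value against the Increments thresholds to pick a low, mid or high material for the cylinder mesh.
; GetSoundPitch walks the same thresholds to choose an entry from SoundPitches, so pickup pitch follows the coin's value tier.
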(event `self.ReceiveActorBeginOverlap`
  (params (OtherActor :type "Actor Object Reference"))
  (bind _value (`self.Value`))
  (bind _asbp_player (cast `/Game/MoTGF/Blueprints/Player/BP_Player` OtherActor))
  (`/Game/MoTGF/Blueprints/Player/BP_Player.AddPendingMoney` _asbp_player _value)
  (bind _pitch (`self.GetSoundPitch` _value))
  (`GameplayStatics.PlaySoundAtLocation` (`AudioComponent.Sound` (`self.PickupSound`)) (`self.K2_GetActorLocation`) (struct) 1.0 _pitch 0.0 null null null null)
  (`self.K2_DestroyActor`))

(event `self.ReceiveTick`
  (params (DeltaSeconds :type "Float (single-precision)"))
  (`self.K2_AddActorWorldRotation` (`KismetMathLibrary.MakeRotator` 0.0 0.0 (* DeltaSeconds 180.0))))

(fn `GetSoundPitch`
  (params (Value :type Integer))
  (returns (Pitch :type "Float (double-precision)"))
  (set `self.PickupPitch` (`|GetArrayItem` (`self.SoundPitches`)))
  (for (_array_element _array_index) (`self.Increments`)
    (if (>= Value _array_element)
      (bind _result (`/Engine/EditorBlueprintResources/StandardMacros.IncrementInt` _array_index)
        (:`  `
          (set `self.PickupPitch` (`|GetArrayItem` (`self.SoundPitches`) _result))))))
  (return (`self.PickupPitch`)))

(fn `UserConstructionScript`
  (if (< (`self.Value`) (`|GetArrayItem` (`self.Increments`)))
    (`PrimitiveComponent.SetMaterial` (`self.Cylinder`) 0 (`self.LowValueMat`)) ; Coin value is less than 1st index value
    (elif (< (`self.Value`) (`|GetArrayItem` (`self.Increments`) 1))
      (`PrimitiveComponent.SetMaterial` (`self.Cylinder`) 0 (`self.MidValueMat`)) ; Coin value is less than 2nd index value
      (else
        (`PrimitiveComponent.SetMaterial` (`self.Cylinder`) 0 (`self.HighValueMat`)) ; Coin value surpasses index values
      ))))