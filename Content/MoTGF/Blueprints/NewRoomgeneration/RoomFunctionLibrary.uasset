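; Blueprint function library for procedural room generation, with helpers for the player pawn check, room manager lookup and three/four-way room check.
; CreateAdjacentRoom removes rooms whose class name contains the direction letter, then returns a random remainder and grid offset.
; Its corner-or-straight roll, RandomInteger(1) == 1, always selects straight rooms.
; The older per-direction getters and branch door-counter functions have unconnected bodies that never run.
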(fn `CreateAdjacentRoom`
  (params (Direction :type "/Game/MoTGF/Blueprints/NewRoomgeneration/Enum_DirectionCompass Enum" :default "NewEnumerator0"))
  (returns (RoomClass :type "/Game/MoTGF/Blueprints/NewRoomgeneration/Rooms/Room_Base Class Reference") (Position :type "Vector Structure"))
  (locals (CornerRooms :type "Array of /Game/MoTGF/Blueprints/NewRoomgeneration/Rooms/Room_Base Class Reference") (StraightRooms :type "Array of /Game/MoTGF/Blueprints/NewRoomgeneration/Rooms/Room_Base Class Reference") (EndRoom_W :type "Actor Class Reference" :default "/Script/Engine.BlueprintGeneratedClass'/Game/MoTGF/Blueprints/NewRoomgeneration/Rooms/Room_1W_W.Room_1W_W_C'") (EndRoom_E :type "Actor Class Reference" :default "/Script/Engine.BlueprintGeneratedClass'/Game/MoTGF/Blueprints/NewRoomgeneration/Rooms/Room_1W_E.Room_1W_E_C'") (EndRoom_S :type "Actor Class Reference" :default "/Script/Engine.BlueprintGeneratedClass'/Game/MoTGF/Blueprints/NewRoomgeneration/Rooms/Room_1W_S.Room_1W_S_C'") (EndRoom_N :type "Actor Class Reference" :default "/Script/Engine.BlueprintGeneratedClass'/Game/MoTGF/Blueprints/NewRoomgeneration/Rooms/Room_1W_N.Room_1W_N_C'") (Rooms :type "Array of /Game/MoTGF/Blueprints/NewRoomgeneration/Rooms/Room_Base Class Reference") (DirectionChar :type String) (NextPos :type "Vector Structure"))
  (bind _rooms (`local.Rooms`))
  (if (== (`KismetMathLibrary.RandomInteger` 1) 1)
    (for _array_element (`local.CornerRooms`)
      (`KismetArrayLibrary.Array_Add` _rooms _array_element))
    (else
      (for _array_element_2 (`local.StraightRooms`)
        (`KismetArrayLibrary.Array_Add` _rooms _array_element_2))))
  (switch `/Game/MoTGF/Blueprints/NewRoomgeneration/Enum_DirectionCompass` Direction
    (:`NewEnumerator0`
      (set `local.DirectionChar` "N")
      (set `local.NextPos` (2000.0 0.0 0.0)))
    (:`NewEnumerator1`
      (set `local.DirectionChar` "S")
      (set `local.NextPos` (-2000.0 0.0 0.0)))
    (:`NewEnumerator2`
      (set `local.DirectionChar` "E")
      (set `local.NextPos` (0.0 2000.0 0.0)))
    (:`NewEnumerator3`
      (set `local.DirectionChar` "W")
      (set `local.NextPos` (0.0 -2000.0 0.0))))
  (for _array_element_3 (`local.Rooms`)
    (if (`KismetStringLibrary.Contains` (`KismetSystemLibrary.GetClassDisplayName` _array_element_3) (`local.DirectionChar`) true)
      (`KismetArrayLibrary.Array_RemoveItem` (`local.Rooms`) _array_element_3)))
  (return (`KismetArrayLibrary.Array_Random` (`local.Rooms`)) (`local.NextPos`)))

(fn `GetBranch`
  (returns (Branch :type Boolean))
  (locals (GameMode :type "Object Object Reference")))

(fn `GetEastRoom`
  (params (Room :type "Actor Object Reference"))
  (returns (SouthRoom :type "Actor Class Reference") (SouthRoomLocation :type "Transform Structure"))
  (locals (EastArray :type "Array of Actor Class Reference") (EastLocation :type "Transform Structure") (EastGameMode :type "Object Object Reference") (StraightEW_1 :type "Array of Actor Class Reference")))

(fn `GetNorthRoom`
  (params (NewParam :type "Actor Object Reference"))
  (returns (SouthRoom :type "Actor Class Reference") (SouthRoomLocation :type "Transform Structure"))
  (locals (NorthArray :type "Array of Actor Class Reference") (NorthGameMode :type "Object Object Reference") (NorthLocation :type "Transform Structure") (StraightNS_0 :type "Array of Actor Class Reference")))

(fn `GetRoomManager`
  (returns (RoomManager :type "/Game/MoTGF/Blueprints/NewRoomgeneration/RoomManager Object Reference"))
  (bind _returnvalue (`GameplayStatics.GetActorOfClass` null "/Game/MoTGF/Blueprints/NewRoomgeneration/RoomManager.RoomManager_C"))
  (return _returnvalue))

(fn `GetSouthRoom`
  (params (NewParam :type "Actor Object Reference"))
  (returns (SouthRoom :type "Actor Class Reference") (SouthRoomLocation :type "Transform Structure"))
  (locals (SouthArray :type "Array of Actor Class Reference") (SouthLocation :type "Transform Structure") (SouthGameMode :type "Object Object Reference") (StraightNS :type "Array of Actor Class Reference")))

(fn `GetWestRoom`
  (params (NewParam :type "Actor Object Reference"))
  (returns (SouthRoom :type "Actor Class Reference") (SouthRoomLocation :type "Transform Structure"))
  (locals (WestArray :type "Array of Actor Class Reference") (GameMode :type "Object Object Reference") (Location :type "Transform Structure") (StraightEW_2 :type "Array of Actor Class Reference")))

(fn `IncrementDoors`
  (locals (GameMode :type "Object Object Reference")))

(fn `IsPlayerPawn`
  (params (Actor :type "Actor Object Reference"))
  (returns (Result :type Boolean))
  (return (== (`GameplayStatics.GetObjectClass` Actor) null)))

(fn `IsThreeOrFourWayRoom`
  (params (Room :type "/Game/MoTGF/Blueprints/NewRoomgeneration/Rooms/Room_Base Class Reference"))
  (returns (Result :type Boolean))
  (locals (`3WayRooms` :type "Array of /Game/MoTGF/Blueprints/NewRoomgeneration/Rooms/Room_Base Class Reference") (`4WayRooms` :type "Array of /Game/MoTGF/Blueprints/NewRoomgeneration/Rooms/Room_Base Class Reference"))
  (return (or (!= (`KismetArrayLibrary.Array_Find` (`local.3WayRooms`) Room) -1) (!= (`KismetArrayLibrary.Array_Find` (`local.4WayRooms`) Room) -1))))