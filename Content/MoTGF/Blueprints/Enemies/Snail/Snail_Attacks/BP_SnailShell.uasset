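; Behavior Tree task that puts a snail enemy into its shell form as one of its attacks.
; It tries casts to the base snail and the Average, Tanky and Speedy bosses in turn, calling ShellForm on the match.
; It binds ShellEnd to the snail's ready-end event but finishes successfully at once, as that handler is empty.
; If no cast matches, the task never calls FinishExecute.
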(event `self.ReceiveExecuteAI`
  (params (OwnerController :type "AIController Object Reference") (ControlledPawn :type "Pawn Object Reference"))
  (bind _asbp_snail (cast `/Game/MoTGF/Blueprints/Enemies/Snail/BP_Snail` ControlledPawn)
    (:`then`
      (`/Game/MoTGF/Blueprints/Enemies/Snail/BP_Snail.Shell Form` _asbp_snail)
      (add `/Game/MoTGF/Blueprints/Enemies/Snail/BP_Snail.OnReadyEnd` _asbp_snail (delegate `ShellEnd`))
      (`self.FinishExecute` true))
    (:`CastFailed`
      (bind _assnail_boss (cast `/Game/MoTGF/Blueprints/Enemies/Boss/SnailBossAverage` ControlledPawn)
        (:`then`
          (`/Game/MoTGF/Blueprints/Enemies/Boss/SnailBossAverage.Shell Form` _assnail_boss)
          (add `/Game/MoTGF/Blueprints/Enemies/Boss/SnailBossAverage.OnReadyEnd` _assnail_boss (delegate `ShellEnd`))
          (`self.FinishExecute` true))
        (:`CastFailed`
          (bind _assnail_boss_tanky (cast `/Game/MoTGF/Blueprints/Enemies/Boss/SnailBossTanky` ControlledPawn)
            (:`then`
              (`/Game/MoTGF/Blueprints/Enemies/Boss/SnailBossTanky.Shell Form` _assnail_boss_tanky)
              (add `/Game/MoTGF/Blueprints/Enemies/Boss/SnailBossTanky.OnReadyEnd` _assnail_boss_tanky (delegate `ShellEnd`))
              (`self.FinishExecute` true))
            (:`CastFailed`
              (bind _assnail_boss_speedy (cast `/Game/MoTGF/Blueprints/Enemies/Boss/SnailBossSpeedy` ControlledPawn))
              (`/Game/MoTGF/Blueprints/Enemies/Boss/SnailBossSpeedy.Shell Form` _assnail_boss_speedy)
              (add `/Game/MoTGF/Blueprints/Enemies/Boss/SnailBossSpeedy.OnReadyEnd` _assnail_boss_speedy (delegate `ShellEnd`))
              (`self.FinishExecute` true))))))))

(event `ShellEnd`)