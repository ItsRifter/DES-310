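; BackgroundMusic is a Blueprint that switches the game's music between a piano track and a boss fight track.
; The custom events BossFightStart and PianoMusic each play their own audio component from the start and set the other's volume multiplier to zero.
; The silenced track is muted without being stopped, and there is no crossfade or automatic trigger in the Blueprint itself.
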(event `self.ReceiveBeginPlay`)

(event `BossFightStart`
  (bind _boss (`self.Boss`))
  (`AudioComponent.Play` _boss 0.0)
  (`AudioComponent.SetVolumeMultiplier` _boss 0.65)
  (`AudioComponent.SetVolumeMultiplier` (`self.Piano`) 0.0))

(event `PianoMusic`
  (bind _piano (`self.Piano`))
  (`AudioComponent.Play` _piano 0.0)
  (`AudioComponent.SetVolumeMultiplier` _piano 0.1)
  (`AudioComponent.SetVolumeMultiplier` (`self.Boss`) 0.0))

(fn `UserConstructionScript`)