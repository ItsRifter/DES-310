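; Health pickup actor that restores one point of health to the player on touch.
; Tick spins it around the yaw axis by a mostly fixed per-frame step, so the rotation speed depends on frame rate.
; Overlapping the Collider with a BP_Player below max health increments CurrentHealth and destroys the item; at full health it stays in the world.
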(event `self.ReceiveTick`
  (params (DeltaSeconds :type "Float (single-precision)"))
  ;[1 1 1] Do spinning rotation
  (`self.K2_AddActorWorldRotation` (`KismetMathLibrary.MakeRotator` 0.0 0.0 (+ (* DeltaSeconds 1.0) 2.5))))

(event `self.Collider.OnComponentBeginOverlap`
  (params (OverlappedComponent :type "PrimitiveComponent Object Reference") (OtherActor :type "Actor Object Reference") (OtherComp :type "PrimitiveComponent Object Reference") (OtherBodyIndex :type Integer) (bFromSweep :type Boolean) (SweepResult :type "HitResult Structure (by ref)"))
  ;[1 1 1] On player collided, give health
  (bind _asbp_player (cast `/Game/MoTGF/Blueprints/Player/BP_Player` OtherActor))
  (bind _currenthealth (`/Game/MoTGF/Blueprints/Player/BP_Player.CurrentHealth` _asbp_player))
  (if (< _currenthealth (`/Game/MoTGF/Blueprints/Player/BP_Player.MaxHealth` _asbp_player))
    (`/Engine/EditorBlueprintResources/StandardMacros.IncrementInt` _currenthealth
      (:`  `
        (`self.K2_DestroyActor`)))))

(fn `UserConstructionScript`)