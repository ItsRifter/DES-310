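; Player Blueprint that handles weapon, inventory and shop interaction input.
; On BeginPlay it adds a BP_Inventory, then spawns a scythe and a spade at the controller's transform and registers both without equipping them.
; Enhanced Input actions attack with ActiveWeapon, switch between four inventory slots, and toggle any overlapping BP_Shop open or closed.
; A debug key stops use of the active weapon.
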(event Input|EnhancedActionEvents|EnhancedInputActionIA_Use
  (params (ActionValue :type Boolean) (ElapsedSeconds :type Float%20%28double-precision%29) (TriggeredSeconds :type Float%20%28double-precision%29) (InputAction :type Input%20Action%20Object%20Reference :default "/Game/David/Input/IA_Use.IA_Use"))
  (:Started
    (for _array_element (Collision|GetOverlappingActors 0 :!class /Script/Engine.Actor)
      (bind _asbp_shop (Utilities|Casting|CastToBP_Shop _array_element))
      (bind _isopen (Default|IsOpen _asbp_shop))
      (if _isopen
        (Default|CloseShop _asbp_shop)
        (else
          (Default|OpenShop _asbp_shop))))))

(event Input|EnhancedActionEvents|EnhancedInputActionIA_Attack
  (params (ActionValue :type Boolean) (ElapsedSeconds :type Float%20%28double-precision%29) (TriggeredSeconds :type Float%20%28double-precision%29) (InputAction :type Input%20Action%20Object%20Reference :default "/Game/David/Input/IA_Attack.IA_Attack"))
  (:Started
    (if (Utilities|IsValid (Variables|Default|GetActiveWeapon))
      (Default|DoAttack (Variables|Default|GetActiveWeapon)))))

(event Input|EnhancedActionEvents|EnhancedInputActionIA_Slot_1
  (params (ActionValue :type Boolean) (ElapsedSeconds :type Float%20%28double-precision%29) (TriggeredSeconds :type Float%20%28double-precision%29) (InputAction :type Input%20Action%20Object%20Reference :default "/Game/David/Input/IA_Slot_1.IA_Slot_1"))
  (:Started
    (Default|ChangeItemfromSlot (Variables|Default|GetInventory) 1)))

(event Input|EnhancedActionEvents|EnhancedInputActionIA_Slot_2
  (params (ActionValue :type Boolean) (ElapsedSeconds :type Float%20%28double-precision%29) (TriggeredSeconds :type Float%20%28double-precision%29) (InputAction :type Input%20Action%20Object%20Reference :default "/Game/David/Input/IA_Slot_2.IA_Slot_2"))
  (:Started
    (Default|ChangeItemfromSlot (Variables|Default|GetInventory) 2)))

(event Input|EnhancedActionEvents|EnhancedInputActionIA_Slot_3
  (params (ActionValue :type Boolean) (ElapsedSeconds :type Float%20%28double-precision%29) (TriggeredSeconds :type Float%20%28double-precision%29) (InputAction :type Input%20Action%20Object%20Reference :default "/Game/David/Input/IA_Slot_3.IA_Slot_3"))
  (:Started
    (Default|ChangeItemfromSlot (Variables|Default|GetInventory) 3)))

(event Input|EnhancedActionEvents|EnhancedInputActionIA_Slot_4
  (params (ActionValue :type Boolean) (ElapsedSeconds :type Float%20%28double-precision%29) (TriggeredSeconds :type Float%20%28double-precision%29) (InputAction :type Input%20Action%20Object%20Reference :default "/Game/David/Input/IA_Slot_4.IA_Slot_4"))
  (:Started
    (Default|ChangeItemfromSlot (Variables|Default|GetInventory) 4)))

(event EventBeginPlay
  (bind _returnvalue (Game|AddComponentbyClass "/Game/David/Blueprints/Player/BP_Inventory.BP_Inventory_C"))
  (Variables|Default|SetInventory _returnvalue)
  (bind _returnvalue_2 (Game|SpawnActorfromClass "/Game/David/Blueprints/Weapons/Weapons/BP_Wep_Scythe.BP_Wep_Scythe_C" (Transformation|GetActorTransform (Pawn|GetController)) "Undefined" "MultiplyWithRoot" 0 0))
  (Default|AddWeapon (Variables|Default|GetInventory) false _returnvalue_2)
  (Default|OnObtain _returnvalue_2 self)
  (bind _returnvalue_3 (Game|SpawnActorfromClass "/Game/David/Blueprints/Weapons/Weapons/BP_Wep_Spade.BP_Wep_Spade_C" (Transformation|GetActorTransform (Pawn|GetController)) "Undefined" "MultiplyWithRoot" 0 0))
  (Default|AddWeapon (Variables|Default|GetInventory) false _returnvalue_3)
  (Default|OnObtain _returnvalue_3 self))

(event Input|KeyboardEvents|DebugKey0
  (params (Key :type Key%20Structure :default "None") (ActionValue :type Input%20Action%20Value%20Structure))
  (:Pressed
    (if (Utilities|IsValid (Variables|Default|GetActiveWeapon))
      (Default|StopUsing (Variables|Default|GetActiveWeapon)))))

(fn ConstructionScript)