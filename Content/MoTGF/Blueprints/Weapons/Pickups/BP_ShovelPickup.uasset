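; BP_ShovelPickup is a weapon pickup for the shovel.
; On BeginPlay it spawns a BP_Wep_Shovel actor and stores it as its weapon reference.
; When an actor begins overlapping its capsule, it passes that actor and the stored weapon to Pickup, whose logic is not defined in this graph.
; A disconnected leftover chain that would add a scythe to the player's inventory never runs.
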(event `self.ReceiveBeginPlay`
  (bind _returnvalue (`|SpawnActorFromClass` "/Game/MoTGF/Blueprints/Weapons/Weapons/Shovel/BP_Wep_Shovel.BP_Wep_Shovel_C" (`KismetMathLibrary.MakeTransform` (0.0 0.0 0.0)) "Undefined" "MultiplyWithRoot" null null))
  (set `self.WeaponBaseRef` _returnvalue))

(event `self.Capsule.OnComponentBeginOverlap`
  (params (OverlappedComponent :type "PrimitiveComponent Object Reference") (OtherActor :type "Actor Object Reference") (OtherComp :type "PrimitiveComponent Object Reference") (OtherBodyIndex :type Integer) (bFromSweep :type Boolean) (SweepResult :type "HitResult Structure (by ref)"))
  (`self.Pickup` OtherActor (`self.WeaponBaseRef`)))

(fn `UserConstructionScript`)