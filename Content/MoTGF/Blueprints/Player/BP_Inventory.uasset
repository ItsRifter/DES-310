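; BP_Inventory is the player's weapon inventory, attached to BP_Player, which it caches by casting its owner on BeginPlay.
; Four slot input actions switch to the matching Weapons array entry, stopping the active weapon, starting the new one and printing its name.
; AddWeapon appends a weapon, starts or stops its use and notifies it of its new owner, without updating the player's ActiveWeapon.
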(event `EnhancedInput|/Game/MoTGF/Blueprints/Input/IA_Slot_1`
  (params (ActionValue :type Boolean) (ElapsedSeconds :type "Float (double-precision)") (TriggeredSeconds :type "Float (double-precision)") (InputAction :type "InputAction Object Reference" :default "/Game/MoTGF/Blueprints/Input/IA_Slot_1.IA_Slot_1"))
  (:`Started`
    (`self.ChangeItemFromSlot` 0)))

(event `self.ReceiveBeginPlay`
  (`self.AssignPlayer`))

(event `EnhancedInput|/Game/MoTGF/Blueprints/Input/IA_Slot_2`
  (params (ActionValue :type Boolean) (ElapsedSeconds :type "Float (double-precision)") (TriggeredSeconds :type "Float (double-precision)") (InputAction :type "InputAction Object Reference" :default "/Game/MoTGF/Blueprints/Input/IA_Slot_2.IA_Slot_2"))
  (:`Started`
    (`self.ChangeItemFromSlot` 1)))

(event `AssignPlayer`
  (bind _asbp_player (cast `/Game/MoTGF/Blueprints/Player/BP_Player` (`self.GetOwner`)))
  (set `self.Player` _asbp_player))

(event `EnhancedInput|/Game/MoTGF/Blueprints/Input/IA_Slot_3`
  (params (ActionValue :type Boolean) (ElapsedSeconds :type "Float (double-precision)") (TriggeredSeconds :type "Float (double-precision)") (InputAction :type "InputAction Object Reference" :default "/Game/MoTGF/Blueprints/Input/IA_Slot_3.IA_Slot_3"))
  (:`Started`
    (`self.ChangeItemFromSlot` 2)))

(event `EnhancedInput|/Game/MoTGF/Blueprints/Input/IA_Slot_4`
  (params (ActionValue :type Boolean) (ElapsedSeconds :type "Float (double-precision)") (TriggeredSeconds :type "Float (double-precision)") (InputAction :type "InputAction Object Reference" :default "/Game/MoTGF/Blueprints/Input/IA_Slot_4.IA_Slot_4"))
  (:`Started`
    (`self.ChangeItemFromSlot` 3)))

(event `ChangeItemFromSlot`
  (params (ToSlot :type Integer))
  (bind _player (`self.Player`))
  (bind _activeweapon (`/Game/MoTGF/Blueprints/Player/BP_Player.ActiveWeapon` _player))
  (bind _output_get (set `self.CurrentSlot` ToSlot))
  (bind _output (`|GetArrayItem` (`self.Weapons`) _output_get))
  (if (`KismetSystemLibrary.IsValid` _output)
    (if (`KismetSystemLibrary.IsValid` _activeweapon)
      (`/Game/MoTGF/Blueprints/Weapons/BP_WeaponBase.StopUsing` _activeweapon))
    (bind _output_get_2 (set `/Game/MoTGF/Blueprints/Player/BP_Player.ActiveWeapon` _output _player))
    (`/Game/MoTGF/Blueprints/Weapons/BP_WeaponBase.StartUsing` _output_get_2)
    (`KismetSystemLibrary.PrintString` (`KismetSystemLibrary.GetDisplayName` _output_get_2))))

(event `AddWeapon`
  (params (ShouldStartUsing :type Boolean) (Weapon :type "/Game/MoTGF/Blueprints/Weapons/BP_WeaponBase Object Reference"))
  ;[1 1 1] Adds weapon to inventory with optional "start using"
  (`KismetArrayLibrary.Array_Add` (`self.Weapons`) Weapon)
  (if ShouldStartUsing
    (`/Game/MoTGF/Blueprints/Weapons/BP_WeaponBase.StartUsing` Weapon)
    (else
      (`/Game/MoTGF/Blueprints/Weapons/BP_WeaponBase.StopUsing` Weapon)))
  (`/Game/MoTGF/Blueprints/Weapons/BP_WeaponBase.OnObtain` Weapon (`self.Player`)))