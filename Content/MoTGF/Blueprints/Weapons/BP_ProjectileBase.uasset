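; BP_ProjectileBase is a base weapon projectile that spawns ahead of the player and travels straight along the player's facing.
; SetupProjectile stores the weapon, ignores player collision and sets direction and lifetime.
; Tick moves it at fixed speed without sweeping, destroying it when lifetime expires.
; Hits on classes listed in IgnoreActors, despite the name, fire OnProjectileCollide and destroy it; the bound handler only prints a placeholder message.
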(event `SetupProjectile`
  (params (FromWeapon :type "/Game/MoTGF/Blueprints/Weapons/BP_WeaponBase Object Reference"))
  (bind _returnvalue (`GameplayStatics.GetPlayerCharacter` 0))
  (bind _returnvalue_2 (`self.K2_GetActorRotation` _returnvalue))
  (set `self.CurLife` (`self.Lifespan`))
  (set `self.Weapon` FromWeapon)
  (`PrimitiveComponent.IgnoreActorWhenMoving` (`self.Collision`) _returnvalue true)
  (`self.K2_SetActorLocation` (+ (`self.K2_GetActorLocation` _returnvalue) (* (`KismetMathLibrary.GetForwardVector` _returnvalue_2) 64.0)))
  (set `self.MoveDir` (`KismetMathLibrary.Conv_RotatorToVector` _returnvalue_2)))

(event `self.ReceiveHit`
  (params (MyComp :type "PrimitiveComponent Object Reference") (Other :type "Actor Object Reference") (OtherComp :type "PrimitiveComponent Object Reference") (bSelfMoved :type Boolean) (HitLocation :type "Vector Structure") (HitNormal :type "Vector Structure") (NormalImpulse :type "Vector Structure") (Hit :type "HitResult Structure (by ref)"))
  (for _array_element (`self.IgnoreActors`) :!label _label
    (if (== _array_element (`GameplayStatics.GetObjectClass` (`.HitActor` (`GameplayStatics.BreakHitResult` Hit))))
      (`self.OnProjectileCollide`)
      (`self.K2_DestroyActor`))))

(event `ProjectileCollided`
  (goto _label :!via `Break`))

(event `self.ReceiveTick`
  (params (DeltaSeconds :type "Float (single-precision)"))
  (`self.K2_AddActorWorldOffset` (* (* DeltaSeconds 192.0) (`self.MoveDir`)))
  (bind _output_get (set `self.CurLife` (- (`self.CurLife`) (* (`GameplayStatics.GetWorldDeltaSeconds`) 1.0))))
  (if (<= _output_get 0.0)
    (`self.K2_DestroyActor`)))

(event `self.ReceiveBeginPlay`
  (add `self.OnProjectileCollide` (delegate `CollectHitTargetsFromProjectile`)))

(event `CollectHitTargetsFromProjectile`
  (`KismetSystemLibrary.PrintString` "Hello"))

(fn `UserConstructionScript`)