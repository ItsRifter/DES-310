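; Behavior tree task that makes a snail enemy or snail boss perform its attack.
; It casts the controlled pawn in turn to BP_Snail and the Average, Speedy and Tanky boss classes, then calls that class's Attack.
; It binds to the pawn's attack-end event but finishes successfully at once, as the AttackEnd handler is empty.
; A pawn matching none of these classes never finishes the task.
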(event `self.ReceiveExecuteAI`
  (params (OwnerController :type "AIController Object Reference") (ControlledPawn :type "Pawn Object Reference"))
  (bind _asbp_snail (cast `/Game/MoTGF/Blueprints/Enemies/Snail/BP_Snail` ControlledPawn)
    (:`then`
      (`/Game/MoTGF/Blueprints/Enemies/Snail/BP_Snail.Attack` _asbp_snail)
      (add `/Game/MoTGF/Blueprints/Enemies/Snail/BP_Snail.OnAttackEnd` _asbp_snail (delegate `AttackEnd`))
      (`self.FinishExecute` true))
    (:`CastFailed`
      (bind _assnail_boss_average (cast `/Game/MoTGF/Blueprints/Enemies/Boss/SnailBossAverage` ControlledPawn)
        (:`then`
          (`/Game/MoTGF/Blueprints/Enemies/Boss/SnailBossAverage.Attack` _assnail_boss_average)
          (add `/Game/MoTGF/Blueprints/Enemies/Boss/SnailBossAverage.OnAttackEnd` _assnail_boss_average (delegate `AttackEnd`))
          (`self.FinishExecute` true))
        (:`CastFailed`
          (bind _assnail_boss_speedy (cast `/Game/MoTGF/Blueprints/Enemies/Boss/SnailBossSpeedy` ControlledPawn)
            (:`then`
              (`/Game/MoTGF/Blueprints/Enemies/Boss/SnailBossSpeedy.Attack` _assnail_boss_speedy)
              (add `/Game/MoTGF/Blueprints/Enemies/Boss/SnailBossSpeedy.OnAttackEnd` _assnail_boss_speedy (delegate `AttackEnd`))
              (`self.FinishExecute` true))
            (:`CastFailed`
              (bind _assnail_boss_tanky (cast `/Game/MoTGF/Blueprints/Enemies/Boss/SnailBossTanky` ControlledPawn))
              (`/Game/MoTGF/Blueprints/Enemies/Boss/SnailBossTanky.Attack` _assnail_boss_tanky)
              (add `/Game/MoTGF/Blueprints/Enemies/Boss/SnailBossTanky.OnAttackEnd` _assnail_boss_tanky (delegate `AttackEnd`))
              (`self.FinishExecute` true))))))))

(event `AttackEnd`)