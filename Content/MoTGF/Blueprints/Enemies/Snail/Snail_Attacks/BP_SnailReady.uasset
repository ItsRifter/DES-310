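; Behavior tree task that puts a snail enemy or snail boss into its Ready attack state.
; It tries casting the controlled pawn to BP_Snail, then the Average, Speedy and Tanky boss variants, calling Ready on the first match.
; It binds the pawn's OnReadyEnd to an empty handler and finishes successfully at once, without waiting for Ready to end.
; If no cast matches, the task never finishes.
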(event `self.ReceiveExecuteAI`
  (params (OwnerController :type "AIController Object Reference") (ControlledPawn :type "Pawn Object Reference"))
  (bind _asbp_snail (cast `/Game/MoTGF/Blueprints/Enemies/Snail/BP_Snail` ControlledPawn)
    (:`then`
      (`/Game/MoTGF/Blueprints/Enemies/Snail/BP_Snail.Ready` _asbp_snail)
      (add `/Game/MoTGF/Blueprints/Enemies/Snail/BP_Snail.OnReadyEnd` _asbp_snail (delegate `ReadyEnd`))
      (`self.FinishExecute` true))
    (:`CastFailed`
      (bind _assnail_boss_average (cast `/Game/MoTGF/Blueprints/Enemies/Boss/SnailBossAverage` ControlledPawn)
        (:`then`
          (`/Game/MoTGF/Blueprints/Enemies/BP_EnemyBase.Ready` _assnail_boss_average)
          (add `/Game/MoTGF/Blueprints/Enemies/Boss/SnailBossAverage.OnReadyEnd` _assnail_boss_average (delegate `ReadyEnd`))
          (`self.FinishExecute` true))
        (:`CastFailed`
          (bind _assnail_boss_speedy (cast `/Game/MoTGF/Blueprints/Enemies/Boss/SnailBossSpeedy` ControlledPawn)
            (:`then`
              (`/Game/MoTGF/Blueprints/Enemies/BP_EnemyBase.Ready` _assnail_boss_speedy)
              (add `/Game/MoTGF/Blueprints/Enemies/Boss/SnailBossSpeedy.OnReadyEnd` _assnail_boss_speedy (delegate `ReadyEnd`))
              (`self.FinishExecute` true))
            (:`CastFailed`
              (bind _assnail_boss_tanky (cast `/Game/MoTGF/Blueprints/Enemies/Boss/SnailBossTanky` ControlledPawn))
              (`/Game/MoTGF/Blueprints/Enemies/BP_EnemyBase.Ready` _assnail_boss_tanky)
              (add `/Game/MoTGF/Blueprints/Enemies/Boss/SnailBossTanky.OnReadyEnd` _assnail_boss_tanky (delegate `ReadyEnd`))
              (`self.FinishExecute` true))))))))

(event `ReadyEnd`)