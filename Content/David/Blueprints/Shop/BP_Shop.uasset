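; BP_Shop is a shop actor that shows a shop menu and holds a randomized list of buyable items.
; It creates the menu widget on BeginPlay and exposes open/close events plus range and open-state queries.
; Tick tracks player overlap and closes the shop when the player leaves.
; ShuffleItems draws up to three unique items from PossibleItems into BuyableItems, capping consecutive failed attempts to avoid endless looping.
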(event `self.ReceiveTick`
  (params (DeltaSeconds :type "Float (single-precision)"))
  (bind _returnvalue (`self.IsOverlappingActor` (`GameplayStatics.GetPlayerCharacter` 0)))
  ;[1 1 1] Player range check
  (set `self.IsPlayerInRange` _returnvalue)
  (if (and (!= _returnvalue true) (== (`self.IsShopOpen`) true))
    (`self.CloseShop`)))

(event `self.ReceiveBeginPlay`
  (bind _returnvalue (`|CreateWidget` "/Game/David/UI/UI_ShopMenu.UI_ShopMenu_C" (`GameplayStatics.GetPlayerController` 0)))
  (set `self.WidgetUI` _returnvalue))

(event `OpenShop`
  (`UserWidget.AddToViewport` (`self.WidgetUI`) 0)
  (set `self.IsShopOpen` true))

(event `CloseShop`
  (`Widget.RemoveFromParent` (`self.WidgetUI`))
  (set `self.IsShopOpen` false))

(event `ShuffleItems`
  (bind _itemstoadd (`self.ItemsToAdd`))
  ;[1 1 1] Shuffle items
  (while (not (or (>= (`KismetArrayLibrary.Array_Length` (`self.ItemsToAdd`)) 3) (>= (`self.ItemAttempts`) (`self.MaxAttempts`))))
    (bind _item (`self.GetRandomItem`))
    (if (`KismetSystemLibrary.IsValidClass` _item)
      (bind _isinstock (`self.HasItemForAdding` _item))
      (if _isinstock
        (`/Engine/EditorBlueprintResources/StandardMacros.IncrementInt` (`self.ItemAttempts`))
        (else
          (`KismetArrayLibrary.Array_Add` (`self.ItemsToAdd`) _item)
          (set `self.HasItemAdded` true)
          (set `self.ItemAttempts` 0)
          (`KismetSystemLibrary.PrintString` (`KismetStringLibrary.Concat_StrStr` (`KismetSystemLibrary.GetClassDisplayName` _item) " was added to the shop") true true (struct :`G` 0.66 :`B` 1.0 :`A` 1.0) 2.5)))
      (else
        (`/Engine/EditorBlueprintResources/StandardMacros.IncrementInt` (`self.ItemAttempts`)))))
  (set `self.BuyableItems` _itemstoadd)
  (`KismetArrayLibrary.Array_Clear` _itemstoadd)
  (if (>= (`self.ItemAttempts`) (`self.MaxAttempts`))
    (`KismetSystemLibrary.PrintString` "Too many attempts were made in getting items"))
  (set `self.ItemAttempts` 0))

(fn `CanUseShop`
  (returns (CanUse :type Boolean))
  (return (`self.IsPlayerInRange`)))

(fn `GetRandomItem`
  (returns (Item :type "Actor Class Reference"))
  (return (`|GetArrayItem` (`self.PossibleItems`) (`KismetMathLibrary.RandomIntegerInRange` 0 (`KismetArrayLibrary.Array_Length` (`self.PossibleItems`))))))

(fn `HasItemForAdding`
  (params (Item :type "Actor Class Reference"))
  (returns (IsInStock :type Boolean))
  (return (!= (`KismetArrayLibrary.Array_Find` (`self.ItemsToAdd`) Item) -1)))

(fn `IsOpen`
  (returns (IsOpen :type Boolean))
  (return (`self.IsShopOpen`)))

(fn `UserConstructionScript`)