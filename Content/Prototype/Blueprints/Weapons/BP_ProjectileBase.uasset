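; Base projectile Blueprint that spawns in front of the player and flies in a straight line until a hit destroys it.
; On BeginPlay it moves itself just ahead of player 0, stores that character's forward vector, and explicitly sets its collision not to ignore the player.
; Tick moves it along that direction at constant speed through unswept world offsets, without a movement component.
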(event `self.ReceiveBeginPlay`
  (bind _returnvalue (`GameplayStatics.GetPlayerCharacter` 0))
  (bind _returnvalue_2 (`self.K2_GetActorRotation` _returnvalue))
  (`PrimitiveComponent.IgnoreActorWhenMoving` (`self.Collision`) _returnvalue false)
  (`self.K2_SetActorLocation` (+ (`self.K2_GetActorLocation` _returnvalue) (* (`KismetMathLibrary.GetForwardVector` _returnvalue_2) 64.0)))
  (set `self.MoveDir` (`KismetMathLibrary.Conv_RotatorToVector` _returnvalue_2)))

(event `self.ReceiveTick`
  (params (DeltaSeconds :type "Float (single-precision)"))
  (`self.K2_AddActorWorldOffset` (* (* DeltaSeconds 192.0) (`self.MoveDir`))))

(event `self.ReceiveHit`
  (params (MyComp :type "PrimitiveComponent Object Reference") (Other :type "Actor Object Reference") (OtherComp :type "PrimitiveComponent Object Reference") (bSelfMoved :type Boolean) (HitLocation :type "Vector Structure") (HitNormal :type "Vector Structure") (NormalImpulse :type "Vector Structure") (Hit :type "HitResult Structure (by ref)"))
  (`self.K2_DestroyActor`))

(fn `UserConstructionScript`)