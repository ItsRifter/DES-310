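; Blueprint function library for procedural room generation, returning room classes and positions on a fixed north/south/east/west grid.
; Directional getters read the GameMode's per-branch door counters: three or more yields a one-way cap, otherwise parity alternates directional and straight pools.
; CreateAdjacentRoom instead picks from corner or straight rooms, filtering by direction letter in class names.
; Helpers increment branch counters, identify the player, find RoomManager and classify three/four-way rooms.
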(fn `CreateAdjacentRoom`
  (params (Direction :type "/Game/MoTGF/Blueprints/RoomGeneration/Enum_DirectionCompass Enum" :default "NewEnumerator0"))
  (returns (RoomClass :type "/Game/MoTGF/Blueprints/RoomGeneration/Rooms/Room_Base Class Reference") (Position :type "Vector Structure"))
  (locals (CornerRooms :type "Array of /Game/MoTGF/Blueprints/RoomGeneration/Rooms/Room_Base Class Reference") (StraightRooms :type "Array of /Game/MoTGF/Blueprints/RoomGeneration/Rooms/Room_Base Class Reference") (EndRoom_W :type "Actor Class Reference" :default "/Script/Engine.BlueprintGeneratedClass'/Game/MoTGF/Blueprints/RoomGeneration/Rooms/Room_1W_W.Room_1W_W_C'") (EndRoom_E :type "Actor Class Reference" :default "/Script/Engine.BlueprintGeneratedClass'/Game/MoTGF/Blueprints/RoomGeneration/Rooms/Room_1W_E.Room_1W_E_C'") (EndRoom_S :type "Actor Class Reference" :default "/Script/Engine.BlueprintGeneratedClass'/Game/MoTGF/Blueprints/RoomGeneration/Rooms/Room_1W_S.Room_1W_S_C'") (EndRoom_N :type "Actor Class Reference" :default "/Script/Engine.BlueprintGeneratedClass'/Game/MoTGF/Blueprints/RoomGeneration/Rooms/Room_1W_N.Room_1W_N_C'") (Rooms :type "Array of /Game/MoTGF/Blueprints/RoomGeneration/Rooms/Room_Base Class Reference") (DirectionChar :type String) (NextPos :type "Vector Structure"))
  (bind _rooms (`local.Rooms`))
  (if (== (`KismetMathLibrary.RandomInteger` 1) 1)
    (for _array_element (`local.CornerRooms`)
      (`KismetArrayLibrary.Array_Add` _rooms _array_element))
    (else
      (for _array_element_2 (`local.StraightRooms`)
        (`KismetArrayLibrary.Array_Add` _rooms _array_element_2))))
  (switch `/Game/MoTGF/Blueprints/RoomGeneration/Enum_DirectionCompass` Direction
    (:`NewEnumerator0`
      (set `local.DirectionChar` "N")
      (set `local.NextPos` (2000.0 0.0 0.0)))
    (:`NewEnumerator1`
      (set `local.DirectionChar` "S")
      (set `local.NextPos` (-2000.0 0.0 0.0)))
    (:`NewEnumerator2`
      (set `local.DirectionChar` "E")
      (set `local.NextPos` (0.0 2000.0 0.0)))
    (:`NewEnumerator3`
      (set `local.DirectionChar` "W")
      (set `local.NextPos` (0.0 -2000.0 0.0))))
  (for _array_element_3 (`local.Rooms`)
    (if (`KismetStringLibrary.Contains` (`KismetSystemLibrary.GetClassDisplayName` _array_element_3) (`local.DirectionChar`) true)
      (`KismetArrayLibrary.Array_RemoveItem` (`local.Rooms`) _array_element_3)))
  (return (`KismetArrayLibrary.Array_Random` (`local.Rooms`)) (`local.NextPos`)))

(fn `GetBranch`
  (returns (Branch :type Boolean))
  (locals (GameMode :type "/Game/MoTGF/Blueprints/Gameplay/MOTGF_Gamemode Object Reference"))
  (bind _asmotgf_gamemode (cast `/Game/MoTGF/Blueprints/Gameplay/MOTGF_Gamemode` (`GameplayStatics.GetGameMode` null)))
  (bind _output_get (set `local.GameMode` _asmotgf_gamemode))
  (return (`/Game/MoTGF/Blueprints/Gameplay/MOTGF_Gamemode.LeftBranch` _output_get)))

(fn `GetEastRoom`
  (params (Room :type "Actor Object Reference"))
  (returns (SouthRoom :type "Actor Class Reference") (SouthRoomLocation :type "Transform Structure"))
  (locals (EastArray :type "Array of Actor Class Reference") (EastLocation :type "Transform Structure") (EastGameMode :type "/Game/MoTGF/Blueprints/Gameplay/MOTGF_Gamemode Object Reference") (StraightEW_1 :type "Array of Actor Class Reference"))
  (bind _eastgamemode (`local.EastGameMode`))
  (bind _output (`|GetArrayItem` (`local.StraightEW_1`) (`KismetMathLibrary.RandomIntegerInRange` 0 (- (`KismetArrayLibrary.Array_Length` (`local.StraightEW_1`)) 1))))
  (bind _asmotgf_gamemode (cast `/Game/MoTGF/Blueprints/Gameplay/MOTGF_Gamemode` (`GameplayStatics.GetGameMode` null)))
  (set `local.EastGameMode` _asmotgf_gamemode)
  (set `local.EastLocation` (`KismetMathLibrary.Conv_VectorToTransform` (+ (`Actor.K2_GetActorLocation` Room) (0.0 2000.0 0.0))))
  (if (`/Game/MoTGF/Blueprints/Gameplay/MOTGF_Gamemode.LeftBranch` (`local.EastGameMode`))
    (if (>= (`/Game/MoTGF/Blueprints/Gameplay/MOTGF_Gamemode.LeftDoorsEntered` _eastgamemode) 3)
      _
      (else
        (if (`/Game/MoTGF/Blueprints/Gameplay/MOTGF_Gamemode.LeftBranch` (`local.EastGameMode`)) :!label _label
          (if (== (mod (`/Game/MoTGF/Blueprints/Gameplay/MOTGF_Gamemode.LeftDoorsEntered` (`local.EastGameMode`)) 2) 0)
            _
            (else
              (return _output (`local.EastLocation`))))
          (elif (== (mod (`/Game/MoTGF/Blueprints/Gameplay/MOTGF_Gamemode.RightDoorsEntered` (`local.EastGameMode`)) 2) 0)
            _
            (else
              (return _output (`local.EastLocation`)))))
        (return (`|GetArrayItem` (`local.EastArray`) (`KismetMathLibrary.RandomIntegerInRange` 0 (- (`KismetArrayLibrary.Array_Length` (`local.EastArray`)) 1))) (`local.EastLocation`))))
    (elif (>= (`/Game/MoTGF/Blueprints/Gameplay/MOTGF_Gamemode.RightDoorsEntered` _eastgamemode) 3)
      _
      (else
        (goto _label))))
  (return "/Game/MoTGF/Blueprints/RoomGeneration/Rooms/Room_1W_W.Room_1W_W_C" (`local.EastLocation`)))

(fn `GetNorthRoom`
  (params (NewParam :type "Actor Object Reference"))
  (returns (SouthRoom :type "Actor Class Reference") (SouthRoomLocation :type "Transform Structure"))
  (locals (NorthArray :type "Array of Actor Class Reference") (NorthGameMode :type "/Game/MoTGF/Blueprints/Gameplay/MOTGF_Gamemode Object Reference") (NorthLocation :type "Transform Structure") (StraightNS_0 :type "Array of Actor Class Reference"))
  (bind _northgamemode (`local.NorthGameMode`))
  (bind _output (`|GetArrayItem` (`local.StraightNS_0`) (`KismetMathLibrary.RandomIntegerInRange` 0 (- (`KismetArrayLibrary.Array_Length` (`local.StraightNS_0`)) 1))))
  (bind _asmotgf_gamemode (cast `/Game/MoTGF/Blueprints/Gameplay/MOTGF_Gamemode` (`GameplayStatics.GetGameMode` null)))
  (set `local.NorthGameMode` _asmotgf_gamemode)
  (set `local.NorthLocation` (`KismetMathLibrary.Conv_VectorToTransform` (+ (`Actor.K2_GetActorLocation` NewParam) (2000.0 0.0 0.0))))
  (if (`/Game/MoTGF/Blueprints/Gameplay/MOTGF_Gamemode.LeftBranch` (`local.NorthGameMode`))
    (if (>= (`/Game/MoTGF/Blueprints/Gameplay/MOTGF_Gamemode.LeftDoorsEntered` _northgamemode) 3)
      _
      (else
        (if (`/Game/MoTGF/Blueprints/Gameplay/MOTGF_Gamemode.LeftBranch` (`local.NorthGameMode`)) :!label _label
          (if (== (mod (`/Game/MoTGF/Blueprints/Gameplay/MOTGF_Gamemode.LeftDoorsEntered` (`local.NorthGameMode`)) 2) 0)
            _
            (else
              (return _output (`local.NorthLocation`))))
          (elif (== (mod (`/Game/MoTGF/Blueprints/Gameplay/MOTGF_Gamemode.RightDoorsEntered` (`local.NorthGameMode`)) 2) 0)
            _
            (else
              (return _output (`local.NorthLocation`)))))
        (return (`|GetArrayItem` (`local.NorthArray`) (`KismetMathLibrary.RandomIntegerInRange` 0 (- (`KismetArrayLibrary.Array_Length` (`local.NorthArray`)) 1))) (`local.NorthLocation`))))
    (elif (>= (`/Game/MoTGF/Blueprints/Gameplay/MOTGF_Gamemode.RightDoorsEntered` _northgamemode) 3)
      _
      (else
        (goto _label))))
  (return "/Game/MoTGF/Blueprints/RoomGeneration/Rooms/Room_1W_S.Room_1W_S_C" (`local.NorthLocation`)))

(fn `GetRoomManager`
  (returns (RoomManager :type "/Game/MoTGF/Blueprints/RoomGeneration/RoomManager Object Reference"))
  (bind _returnvalue (`GameplayStatics.GetActorOfClass` null "/Game/MoTGF/Blueprints/RoomGeneration/RoomManager.RoomManager_C"))
  (return _returnvalue))

(fn `GetSouthRoom`
  (params (NewParam :type "Actor Object Reference"))
  (returns (SouthRoom :type "Actor Class Reference") (SouthRoomLocation :type "Transform Structure"))
  (locals (SouthArray :type "Array of Actor Class Reference") (SouthLocation :type "Transform Structure") (SouthGameMode :type "/Game/MoTGF/Blueprints/Gameplay/MOTGF_Gamemode Object Reference") (StraightNS :type "Array of Actor Class Reference"))
  (bind _southgamemode (`local.SouthGameMode`))
  (bind _output (`|GetArrayItem` (`local.StraightNS`) (`KismetMathLibrary.RandomIntegerInRange` 0 (- (`KismetArrayLibrary.Array_Length` (`local.StraightNS`)) 1))))
  (bind _asmotgf_gamemode (cast `/Game/MoTGF/Blueprints/Gameplay/MOTGF_Gamemode` (`GameplayStatics.GetGameMode` null)))
  (set `local.SouthGameMode` _asmotgf_gamemode)
  (set `local.SouthLocation` (`KismetMathLibrary.Conv_VectorToTransform` (+ (`Actor.K2_GetActorLocation` NewParam) (-2000.0 0.0 0.0))))
  (if (`/Game/MoTGF/Blueprints/Gameplay/MOTGF_Gamemode.LeftBranch` (`local.SouthGameMode`))
    (if (>= (`/Game/MoTGF/Blueprints/Gameplay/MOTGF_Gamemode.LeftDoorsEntered` _southgamemode) 3)
      _
      (else
        (if (`/Game/MoTGF/Blueprints/Gameplay/MOTGF_Gamemode.LeftBranch` (`local.SouthGameMode`)) :!label _label
          (if (== (mod (`/Game/MoTGF/Blueprints/Gameplay/MOTGF_Gamemode.LeftDoorsEntered` (`local.SouthGameMode`)) 2) 0)
            _
            (else
              (return _output (`local.SouthLocation`))))
          (elif (== (mod (`/Game/MoTGF/Blueprints/Gameplay/MOTGF_Gamemode.RightDoorsEntered` (`local.SouthGameMode`)) 2) 0)
            _
            (else
              (return _output (`local.SouthLocation`)))))
        (return (`|GetArrayItem` (`local.SouthArray`) (`KismetMathLibrary.RandomIntegerInRange` 0 (- (`KismetArrayLibrary.Array_Length` (`local.SouthArray`)) 1))) (`local.SouthLocation`))))
    (elif (>= (`/Game/MoTGF/Blueprints/Gameplay/MOTGF_Gamemode.RightDoorsEntered` _southgamemode) 3)
      _
      (else
        (goto _label))))
  (return "/Game/MoTGF/Blueprints/RoomGeneration/Rooms/Room_1W_N.Room_1W_N_C" (`local.SouthLocation`)))

(fn `GetWestRoom`
  (params (NewParam :type "Actor Object Reference"))
  (returns (SouthRoom :type "Actor Class Reference") (SouthRoomLocation :type "Transform Structure"))
  (locals (WestArray :type "Array of Actor Class Reference") (GameMode :type "/Game/MoTGF/Blueprints/Gameplay/MOTGF_Gamemode Object Reference") (Location :type "Transform Structure") (StraightEW_2 :type "Array of Actor Class Reference"))
  (bind _gamemode (`local.GameMode`))
  (bind _output (`|GetArrayItem` (`local.StraightEW_2`) (`KismetMathLibrary.RandomIntegerInRange` 0 (- (`KismetArrayLibrary.Array_Length` (`local.StraightEW_2`)) 1))))
  (bind _asmotgf_gamemode (cast `/Game/MoTGF/Blueprints/Gameplay/MOTGF_Gamemode` (`GameplayStatics.GetGameMode` null)))
  (bind _output_get (set `local.GameMode` _asmotgf_gamemode))
  (set `local.Location` (`KismetMathLibrary.Conv_VectorToTransform` (+ (`Actor.K2_GetActorLocation` NewParam) (0.0 -2000.0 0.0))))
  (if (`/Game/MoTGF/Blueprints/Gameplay/MOTGF_Gamemode.LeftBranch` _output_get)
    (if (>= (`/Game/MoTGF/Blueprints/Gameplay/MOTGF_Gamemode.LeftDoorsEntered` _gamemode) 3)
      _
      (else
        (if (`/Game/MoTGF/Blueprints/Gameplay/MOTGF_Gamemode.LeftBranch` (`local.GameMode`)) :!label _label
          (if (== (mod (`/Game/MoTGF/Blueprints/Gameplay/MOTGF_Gamemode.LeftDoorsEntered` (`local.GameMode`)) 2) 0)
            _
            (else
              (return _output (`local.Location`))))
          (elif (== (mod (`/Game/MoTGF/Blueprints/Gameplay/MOTGF_Gamemode.RightDoorsEntered` (`local.GameMode`)) 2) 0)
            _
            (else
              (return _output (`local.Location`)))))
        (return (`|GetArrayItem` (`local.WestArray`) (`KismetMathLibrary.RandomIntegerInRange` 0 (- (`KismetArrayLibrary.Array_Length` (`local.WestArray`)) 1))) (`local.Location`))))
    (elif (>= (`/Game/MoTGF/Blueprints/Gameplay/MOTGF_Gamemode.RightDoorsEntered` _gamemode) 3)
      _
      (else
        (goto _label))))
  (return "/Game/MoTGF/Blueprints/RoomGeneration/Rooms/Room_1W_E.Room_1W_E_C" (`local.Location`)))

(fn `IncrementDoors`
  (locals (GameMode :type "/Game/MoTGF/Blueprints/Gameplay/MOTGF_Gamemode Object Reference"))
  (bind _gamemode (`local.GameMode`))
  (bind _asmotgf_gamemode (cast `/Game/MoTGF/Blueprints/Gameplay/MOTGF_Gamemode` (`GameplayStatics.GetGameMode` null)))
  (bind _output_get (set `local.GameMode` _asmotgf_gamemode))
  (bind _branch (`self.GetBranch` _output_get))
  (if _branch
    (bind _result (`/Engine/EditorBlueprintResources/StandardMacros.IncrementInt` (`/Game/MoTGF/Blueprints/Gameplay/MOTGF_Gamemode.LeftDoorsEntered` _gamemode))
      (:`  `
        (set `/Game/MoTGF/Blueprints/Gameplay/MOTGF_Gamemode.LeftDoorsEntered` _result (`local.GameMode`))))
    (else
      (bind _result_2 (`/Engine/EditorBlueprintResources/StandardMacros.IncrementInt` (`/Game/MoTGF/Blueprints/Gameplay/MOTGF_Gamemode.RightDoorsEntered` _gamemode))
        (:`  `
          (set `/Game/MoTGF/Blueprints/Gameplay/MOTGF_Gamemode.RightDoorsEntered` _result_2 (`local.GameMode`)))))))

(fn `IsPlayerPawn`
  (params (Actor :type "Actor Object Reference"))
  (returns (Result :type Boolean))
  (return (== (`GameplayStatics.GetObjectClass` Actor) "/Game/MoTGF/Blueprints/Player/BP_Player.BP_Player_C")))

(fn `IsThreeOrFourWayRoom`
  (params (Room :type "/Game/MoTGF/Blueprints/RoomGeneration/Rooms/Room_Base Class Reference"))
  (returns (Result :type Boolean))
  (locals (`3WayRooms` :type "Array of /Game/MoTGF/Blueprints/RoomGeneration/Rooms/Room_Base Class Reference") (`4WayRooms` :type "Array of /Game/MoTGF/Blueprints/RoomGeneration/Rooms/Room_Base Class Reference"))
  (return (or (!= (`KismetArrayLibrary.Array_Find` (`local.3WayRooms`) Room) -1) (!= (`KismetArrayLibrary.Array_Find` (`local.4WayRooms`) Room) -1))))