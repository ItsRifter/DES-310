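; Player controller that sets up Enhanced Input and drives movement of the player pawn.
; On BeginPlay it adds the IMC_PlayerInput mapping context, then caches PlayerRef through GetPlayerRef on the player character and prints its name.
; Four directional input actions each feed AddMovementInput on player pawn 0, using fixed world-axis vectors scaled by PlayerRef's Speed.
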(event `self.ReceiveBeginPlay`
  (bind _returnvalue (subsystem `EnhancedInputLocalPlayerSubsystem`))
  (`/Engine/EditorBlueprintResources/StandardMacros.IsValid` _returnvalue
    (:`Is Valid`
      (`EnhancedInputSubsystemInterface.AddMappingContext` _returnvalue "/Game/Prototype/Input/IMC_PlayerInput.IMC_PlayerInput" 0 (struct))
      (bind _playerref (`/Engine/EditorBlueprintResources/StandardMacros.GetPlayerRef` (`GameplayStatics.GetPlayerCharacter` 0))
        (:`Result`
          (bind _output_get (set `self.PlayerRef` _playerref))
          (`KismetSystemLibrary.PrintString` (`KismetSystemLibrary.GetDisplayName` _output_get)))))))

(event `EnhancedInput|/Game/Prototype/Input/IA_Movement_Horizontal_Right`
  (params (ActionValue :type Boolean) (ElapsedSeconds :type "Float (double-precision)") (TriggeredSeconds :type "Float (double-precision)") (InputAction :type "InputAction Object Reference" :default "/Game/Prototype/Input/IA_Movement_Horizontal_Right.IA_Movement_Horizontal_Right"))
  (:`Triggered`
    (`Pawn.AddMovementInput` (`GameplayStatics.GetPlayerPawn` 0) (* (`KismetMathLibrary.Vector_Right`) (`/Game/Prototype/Blueprints/Player/BP_Player.Speed` (`self.PlayerRef`))) 1.0 false)))

(event `EnhancedInput|/Game/Prototype/Input/IA_Movement_Horizontal_Left`
  (params (ActionValue :type Boolean) (ElapsedSeconds :type "Float (double-precision)") (TriggeredSeconds :type "Float (double-precision)") (InputAction :type "InputAction Object Reference" :default "/Game/Prototype/Input/IA_Movement_Horizontal_Left.IA_Movement_Horizontal_Left"))
  (:`Triggered`
    (`Pawn.AddMovementInput` (`GameplayStatics.GetPlayerPawn` 0) (* (`KismetMathLibrary.Vector_Left`) (`/Game/Prototype/Blueprints/Player/BP_Player.Speed` (`self.PlayerRef`))) 1.0 false)))

(event `EnhancedInput|/Game/Prototype/Input/IA_Movement_Vertical_Up`
  (params (ActionValue :type Boolean) (ElapsedSeconds :type "Float (double-precision)") (TriggeredSeconds :type "Float (double-precision)") (InputAction :type "InputAction Object Reference" :default "/Game/Prototype/Input/IA_Movement_Vertical_Up.IA_Movement_Vertical_Up"))
  (:`Triggered`
    (`Pawn.AddMovementInput` (`GameplayStatics.GetPlayerPawn` 0) (* (`KismetMathLibrary.Vector_Forward`) (`/Game/Prototype/Blueprints/Player/BP_Player.Speed` (`self.PlayerRef`))) 1.0 false)))

(event `EnhancedInput|/Game/Prototype/Input/IA_Movement_Vertical_Down`
  (params (ActionValue :type Boolean) (ElapsedSeconds :type "Float (double-precision)") (TriggeredSeconds :type "Float (double-precision)") (InputAction :type "InputAction Object Reference" :default "/Game/Prototype/Input/IA_Movement_Vertical_Down.IA_Movement_Vertical_Down"))
  (:`Triggered`
    (`Pawn.AddMovementInput` (`GameplayStatics.GetPlayerPawn` 0) (* (`KismetMathLibrary.Vector_Backward`) (`/Game/Prototype/Blueprints/Player/BP_Player.Speed` (`self.PlayerRef`))) 1.0 false)))

(fn `UserConstructionScript`)