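; BP_Wep_Spade is a prototype melee spade weapon built on a parent weapon class.
; When use starts, it attaches to the player actor and snaps to the location and rotation of the player's Holder component.
; Its attack runs an arc attack driven by step, arc distance and range variables.
; The following check on hit targets leads to no action, and the node that clears them is unconnected.
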(event `self.StartUsing`
  (bind _holder (`/Game/Prototype/Blueprints/Player/BP_Player.Holder` (`self.Player`)))
  (`self.K2_AttachToActor` (`self.Player`) "None" "KeepRelative" "KeepRelative" "KeepRelative" false)
  (`self.K2_SetActorLocationAndRotation` (`SceneComponent.K2_GetComponentLocation` _holder) (`SceneComponent.K2_GetComponentRotation` _holder)))

(event `self.ReceiveBeginPlay`
  (`parent.ReceiveBeginPlay`))

(event `self.OnObtain`
  (params (Player :type "/Game/Prototype/Blueprints/Player/BP_Player Object Reference"))
  (`parent.OnObtain` Player))

(event `self.DoAttack`
  (`self.DoArcAttack` (`self.Steps`) (`self.ArcDistance`) (`self.Range`))
  (if (`KismetArrayLibrary.Array_IsNotEmpty` (`self.HitTargets`))
    _))

(fn `UserConstructionScript`
  (`parent.UserConstructionScript`))