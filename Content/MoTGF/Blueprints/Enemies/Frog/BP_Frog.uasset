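; Frog enemy that winds up and lashes the player with a tongue grapple, built on a parent enemy's attack events.
; It turns toward the player until a grapple lands, and its charge sound's pitch scales inversely with windup time.
; The attack montage leads into a pawn line trace and facing-angle check.
; A hit deals damage and briefly shows a Cable component attached to the player's mesh socket before signalling attack end.
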(event `self.TryDoAttacks`
  (bind _result (`self.CanDoAttack`))
  (if (and _result (not (`self.IsPerformingAttack`)))
    (`self.SetAttackValue` true)))

(event `self.StartAttack`
  (set `self.IsPerformingAttack` true))

(event `self.DoChargingAttack`
  (`self.K2_SetActorRotation` (`KismetMathLibrary.FindLookAtRotation` (`self.K2_GetActorLocation`) (`self.K2_GetActorLocation` (`GameplayStatics.GetPlayerCharacter` 0))))
  (`self.DoPlaySound` (`self.ChargeSound`) (/ 1.0 (`self.AttackChargeTime`)))
  (`|PlayMontage` (`self.Mesh`) "/Game/MoTGF/Animations/Frog/Anim_Frog_Attack_Windup.Anim_Frog_Attack_Windup"
    (:`then`
      (`parent.DoChargingAttack`))))

(event `self.FinishAttack`
  (`parent.FinishAttack`)
  (set `self.IsPerformingAttack` false))

(event `self.ReceiveTick`
  (params (DeltaSeconds :type "Float (single-precision)"))
  (`parent.ReceiveTick` DeltaSeconds)
  (if (not (`self.PlayerGrappled?`))
    (`SceneComponent.SetVisibility` (`self.Cable`) false false)
    (bind _asbp_top_down_character (cast `/Game/TopDown/Blueprints/BP_TopDownCharacter` (`GameplayStatics.GetPlayerCharacter` 0)))
    (`self.K2_SetActorRotation` (`KismetMathLibrary.FindRelativeLookAtRotation` (`KismetMathLibrary.Conv_VectorToTransform` (`self.K2_GetActorLocation`)) (`self.K2_GetActorLocation` _asbp_top_down_character)))))

(event `self.DoAttack`
  (bind _returnvalue (`self.K2_GetActorLocation` (`GameplayStatics.GetPlayerCharacter` 0)))
  (if (not (`self.IsDead`))
    (set `self.IsAttackCharging` false)
    (`|PlayMontage` (`self.Mesh`) "/Game/MoTGF/Animations/Frog/Anim_Frog_Attack.Anim_Frog_Attack"
      (:`then`
        (bind _outhit (`KismetSystemLibrary.LineTraceSingleForObjects` (`self.K2_GetActorLocation`) _returnvalue (`|MakeArray` "ObjectTypeQuery3" :!type "EObjectTypeQuery Enum")))
        (bind (_bblockinghit _binitialoverlap _time _distance _location _impactpoint _normal _impactnormal _physmat _hitactor) (`GameplayStatics.BreakHitResult` _outhit))
        (bind _asbp_player (cast `/Game/MoTGF/Blueprints/Player/BP_Player` _hitactor))
        (set `self.Hit Actor` _asbp_player)
        (if (< (`KismetMathLibrary.DegAcos` (`KismetMathLibrary.Dot_VectorVector` (`KismetMathLibrary.Normal` (- _returnvalue (`self.K2_GetActorLocation`))) (`KismetMathLibrary.GetForwardVector` (`self.K2_GetActorRotation`)))) (`self.AttackAngle`))
          (set `self.Impact Point` _impactpoint)
          (set `self.PlayerGrappled?` true)
          (bind _asbp_player_2 (cast `/Game/MoTGF/Blueprints/Player/BP_Player` (`self.Hit Actor`)))
          (`self.DoPlaySound` (`self.HitSound`) 0.6)
          (`GameplayStatics.ApplyDamage` _asbp_player_2 1.0)
          (`CableComponent.SetAttachEndToComponent` (`self.Cable`) (`Character.Mesh` _asbp_player_2) "FrogSocket")
          (`SceneComponent.SetVisibility` (`self.Cable`) true false)
          (`KismetSystemLibrary.Delay` 1.0)
          (`SceneComponent.SetVisibility` (`self.Cable`) false false)
          (`self.OnAttackEnd`))))))

(event `self.ReceiveAnyDamage`
  (params (Damage :type "Float (single-precision)") (DamageType :type "DamageType Object Reference") (InstigatedBy :type "Controller Object Reference") (DamageCauser :type "Actor Object Reference"))
  (`parent.ReceiveAnyDamage` Damage null null null))

(event `self.Ready`
  (`|PlayMontage` (`self.Mesh`)))

(event `self.ReceiveBeginPlay`
  (`parent.ReceiveBeginPlay`))

(fn `UserConstructionScript`)