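; BP_Wep_Scythe is a scythe weapon Blueprint that performs radius attacks and extends a parent weapon class.
; When obtained, it runs the parent logic and attaches to the owner mesh's WristSocket with relative transform rules.
; DoAttack checks CanAttack, then calls DoRadiusAttack with the charge-attack flag and applies the cooldown.
; BeginPlay and the construction script only defer to the parent.
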(event `self.ReceiveBeginPlay`
  (`parent.ReceiveBeginPlay`))

(event `self.OnObtain`
  (params (Owner :type "/Game/MoTGF/Blueprints/Player/BP_Player Object Reference"))
  (`parent.OnObtain` Owner)
  (`self.K2_AttachToComponent` (`Character.Mesh` Owner) "WristSocket" "KeepRelative" "KeepRelative" "KeepRelative"))

(event `self.DoAttack`
  (params (doChargeAttack :type Boolean))
  (bind _canattack_ (`self.CanAttack`))
  (if _canattack_
    (`self.DoRadiusAttack` doChargeAttack)
    (`self.ApplyCooldown`)))

(fn `UserConstructionScript`
  (`parent.UserConstructionScript`))