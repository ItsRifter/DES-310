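; Gnome enemy Blueprint that attacks the player and dances once the player's health runs out.
; Attack, Ready and Pause events play montages and fire their end callbacks without waiting for completion; Attack also damages the player with no range check.
; Tick watches player health to set the dance flag on the anim Blueprint.
; BeginPlay caches the health-bar widget, then runs parent logic, which also handles incoming damage.
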(event `self.ReceiveTick`
  (params (DeltaSeconds :type "Float (single-precision)"))
  (bind _asbp_player (cast `/Game/MoTGF/Blueprints/Player/BP_Player` (`GameplayStatics.GetPlayerCharacter` 0)))
  (if (<= (`/Game/MoTGF/Blueprints/Player/BP_Player.CurrentHealth` _asbp_player) 0)
    (bind _asgnome_anim_blueprint (cast `/Game/MoTGF/Animations/TEST/GnomeAnimBlueprint` (`SkeletalMeshComponent.GetAnimInstance` (`self.Mesh`))))
    (set `/Game/MoTGF/Animations/TEST/GnomeAnimBlueprint.DoDance` true _asgnome_anim_blueprint)))

(event `self.ReceiveBeginPlay`
  (bind _asbp_enemy_health_ui (cast `/Game/MoTGF/Blueprints/UI/BP_EnemyHealthUI` (`WidgetComponent.GetUserWidgetObject` (`self.Health`))))
  (set `self.BPHealthUI` _asbp_enemy_health_ui)
  (`parent.ReceiveBeginPlay`))

(event `Attack`
  (`KismetSystemLibrary.PrintString` "ATTACK")
  (`|PlayMontage` (`self.Mesh`)
    (:`then`
      (bind _asbp_player (cast `/Game/MoTGF/Blueprints/Player/BP_Player` (`GameplayStatics.GetPlayerPawn` 0)))
      (`GameplayStatics.ApplyDamage` _asbp_player 1.0)
      (`self.OnAttackEnd`))))

(event `Ready`
  (`KismetSystemLibrary.PrintString` "READY")
  (`|PlayMontage` (`self.Mesh`)
    (:`then`
      (`self.OnReadyEnd`))))

(event `Pause`
  (`KismetSystemLibrary.PrintString` "READY")
  (`|PlayMontage` (`self.Mesh`)
    (:`then`
      (`self.OnPauseEnd`))))

(event `self.ReceiveAnyDamage`
  (params (Damage :type "Float (single-precision)") (DamageType :type "DamageType Object Reference") (InstigatedBy :type "Controller Object Reference") (DamageCauser :type "Actor Object Reference"))
  (`parent.ReceiveAnyDamage` Damage null null null))

(fn `UserConstructionScript`)