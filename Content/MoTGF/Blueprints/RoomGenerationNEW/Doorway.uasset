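; Doorway actor for room generation that acts as a lockable door with a player trigger, starting unlocked.
; Lock and Unlock toggle the door mesh's visibility and collision, while AssignRoom stores a room reference and arms the trigger.
; Player overlaps drive a DoOnce that sets HasTriggered and a short cooldown counted down on Tick.
; The file caches the RoomManager but never calls it or the assigned room.
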(event `self.ReceiveBeginPlay`
  (`self.Unlock`)
  (bind _returnvalue (`GameplayStatics.GetActorOfClass` "/Game/MoTGF/Blueprints/RoomGenerationNEW/RoomManager.RoomManager_C"))
  (set `self.RoomManager` _returnvalue))

(event `Lock`
  (set `self.IsLocked` true)
  (`SceneComponent.SetVisibility` (`self.DoorMesh`) true true)
  (`PrimitiveComponent.SetCollisionEnabled` (`self.DoorMesh`) "QueryAndPhysics"))

(event `Unlock`
  (set `self.IsLocked` false)
  (`SceneComponent.SetVisibility` (`self.DoorMesh`) false true)
  (`PrimitiveComponent.SetCollisionEnabled` (`self.DoorMesh`) "NoCollision"))

(event `self.ReceiveTick`
  (params (DeltaSeconds :type "Float (single-precision)"))
  (if (> (`self.WaitTime`) 0.0)
    (set `self.WaitTime` (- (`self.WaitTime`) (* DeltaSeconds 1.0)))))

(event `AssignRoom`
  (params (RoomRef :type "/Game/MoTGF/Blueprints/RoomGenerationNEW/Rooms/Room_Base Object Reference"))
  (set `self.AssignedRoom` RoomRef)
  (set `self.CanBeTriggered` true))

(event `self.TriggerBox.OnComponentEndOverlap`
  (params (OverlappedComponent :type "PrimitiveComponent Object Reference") (OtherActor :type "Actor Object Reference") (OtherComp :type "PrimitiveComponent Object Reference") (OtherBodyIndex :type Integer))
  (bind _result (`/Game/MoTGF/Blueprints/RoomGenerationNEW/RoomFunctionLibrary.IsPlayerPawn` OtherActor))
  (if _result
    (if (`self.CanBeTriggered`)
      (goto _label :!via `Reset`)
      (elif (not (> (`self.WaitTime`) 0.0))
        (set `self.HasTriggered` false)))))

(event `self.TriggerBox.OnComponentBeginOverlap`
  (params (OverlappedComponent :type "PrimitiveComponent Object Reference") (OtherActor :type "Actor Object Reference") (OtherComp :type "PrimitiveComponent Object Reference") (OtherBodyIndex :type Integer) (bFromSweep :type Boolean) (SweepResult :type "HitResult Structure (by ref)"))
  (if (`KismetSystemLibrary.IsValid` (`self.AssignedRoom`))
    (if (not (`self.HasTriggered`))
      (bind _result (`/Game/MoTGF/Blueprints/RoomGenerationNEW/RoomFunctionLibrary.IsPlayerPawn` OtherActor))
      (`/Engine/EditorBlueprintResources/StandardMacros.DoOnce` false :!label _label
        (:`Completed`
          (if _result
            (set `self.HasTriggered` true)
            (set `self.WaitTime` 2.0)))))))

(fn `UserConstructionScript`)