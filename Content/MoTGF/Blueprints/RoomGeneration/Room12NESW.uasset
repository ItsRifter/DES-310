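; Room blueprint with doors on all four sides that grows a procedurally generated layout as the player moves through it.
; The first door the player overlaps is treated as the entrance: it sets FirstDoorEntered and is destroyed.
; Each later door spawns the room class and transform returned by its directional Get…Room call, calls IncrementDoors, then destroys itself.
; An older random-pick south spawn is left disconnected.
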(event `self.NorthDoor.OnComponentBeginOverlap`
  (params (OverlappedComponent :type "PrimitiveComponent Object Reference") (OtherActor :type "Actor Object Reference") (OtherComp :type "PrimitiveComponent Object Reference") (OtherBodyIndex :type Integer) (bFromSweep :type Boolean) (SweepResult :type "HitResult Structure (by ref)"))
  (cast `/Game/MoTGF/Blueprints/Player/BP_Player` OtherActor)
  (if (`self.FirstDoorEntered`)
    (bind (_southroom _southroomlocation) (`/Game/MoTGF/Blueprints/RoomGeneration/RoomFuntionLibra.GetNorthRoom` self))
    (`|SpawnActorFromClass` _southroom _southroomlocation "Undefined" "MultiplyWithRoot" null null)
    (`/Game/MoTGF/Blueprints/RoomGeneration/RoomFuntionLibra.IncrementDoors`)
    (`ActorComponent.K2_DestroyComponent` (`self.NorthDoor`))
    (else
      (set `self.FirstDoorEntered` true)
      (`ActorComponent.K2_DestroyComponent` (`self.NorthDoor`))
      (`KismetSystemLibrary.PrintString` "North destroyed"))))

(event `self.EastDoor.OnComponentBeginOverlap`
  (params (OverlappedComponent :type "PrimitiveComponent Object Reference") (OtherActor :type "Actor Object Reference") (OtherComp :type "PrimitiveComponent Object Reference") (OtherBodyIndex :type Integer) (bFromSweep :type Boolean) (SweepResult :type "HitResult Structure (by ref)"))
  (cast `/Game/MoTGF/Blueprints/Player/BP_Player` OtherActor)
  (if (`self.FirstDoorEntered`)
    (bind (_southroom _southroomlocation) (`/Game/MoTGF/Blueprints/RoomGeneration/RoomFuntionLibra.GetEastRoom` self))
    (`|SpawnActorFromClass` _southroom _southroomlocation "Undefined" "MultiplyWithRoot" null null)
    (`/Game/MoTGF/Blueprints/RoomGeneration/RoomFuntionLibra.IncrementDoors`)
    (`ActorComponent.K2_DestroyComponent` (`self.EastDoor`))
    (else
      (set `self.FirstDoorEntered` true)
      (`ActorComponent.K2_DestroyComponent` (`self.EastDoor`))
      (`KismetSystemLibrary.PrintString` "East destroyed"))))

(event `self.SouthDoor.OnComponentBeginOverlap`
  (params (OverlappedComponent :type "PrimitiveComponent Object Reference") (OtherActor :type "Actor Object Reference") (OtherComp :type "PrimitiveComponent Object Reference") (OtherBodyIndex :type Integer) (bFromSweep :type Boolean) (SweepResult :type "HitResult Structure (by ref)"))
  (cast `/Game/MoTGF/Blueprints/Player/BP_Player` OtherActor)
  (if (`self.FirstDoorEntered`)
    (bind (_southroom _southroomlocation) (`/Game/MoTGF/Blueprints/RoomGeneration/RoomFuntionLibra.GetSouthRoom` self))
    (`|SpawnActorFromClass` _southroom _southroomlocation "Undefined" "MultiplyWithRoot" null null)
    (`/Game/MoTGF/Blueprints/RoomGeneration/RoomFuntionLibra.IncrementDoors`)
    (`ActorComponent.K2_DestroyComponent` (`self.SouthDoor`))
    (else
      (set `self.FirstDoorEntered` true)
      (`ActorComponent.K2_DestroyComponent` (`self.SouthDoor`))
      (`KismetSystemLibrary.PrintString` "South desroyed"))))

(event `self.WestDoor.OnComponentBeginOverlap`
  (params (OverlappedComponent :type "PrimitiveComponent Object Reference") (OtherActor :type "Actor Object Reference") (OtherComp :type "PrimitiveComponent Object Reference") (OtherBodyIndex :type Integer) (bFromSweep :type Boolean) (SweepResult :type "HitResult Structure (by ref)"))
  (cast `/Game/MoTGF/Blueprints/Player/BP_Player` OtherActor)
  (if (`self.FirstDoorEntered`)
    (bind (_southroom _southroomlocation) (`/Game/MoTGF/Blueprints/RoomGeneration/RoomFuntionLibra.GetWestRoom` self))
    (`|SpawnActorFromClass` _southroom _southroomlocation "Undefined" "MultiplyWithRoot" null null)
    (`/Game/MoTGF/Blueprints/RoomGeneration/RoomFuntionLibra.IncrementDoors`)
    (`ActorComponent.K2_DestroyComponent` (`self.WestDoor`))
    (else
      (set `self.FirstDoorEntered` true)
      (`ActorComponent.K2_DestroyComponent` (`self.WestDoor`))
      (`KismetSystemLibrary.PrintString` "West destroyed"))))

(fn `UserConstructionScript`)