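; Behavior Tree task that puts a gnome enemy into its Ready state and backs it away from the player.
; It calls Ready on the gnome, lowers walk speed and issues an AI move to a point a short distance directly opposite the player at the gnome's height.
; It then raises walk speed, waits briefly, binds an empty ReadyEnd handler and finishes successfully.
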(event `self.ReceiveExecuteAI`
  (params (OwnerController :type "AIController Object Reference") (ControlledPawn :type "Pawn Object Reference"))
  (bind _asbp_gnome (cast `/Game/MoTGF/Blueprints/Enemies/Gnome/BP_Gnome` ControlledPawn))
  (`/Game/MoTGF/Blueprints/Enemies/Gnome/BP_Gnome.Ready` _asbp_gnome)
  (set `CharacterMovementComponent.MaxWalkSpeed` 250.0 (`Character.CharacterMovement` _asbp_gnome))
  (bind _returnvalue (`Actor.K2_GetActorLocation` _asbp_gnome))
  (`|AIMoveTo` _asbp_gnome (`KismetMathLibrary.MakeVector` (.x (+ _returnvalue (* (`KismetMathLibrary.GetForwardVector` (`KismetMathLibrary.FindLookAtRotation` _returnvalue (`Actor.K2_GetActorLocation` (`GameplayStatics.GetPlayerCharacter` 0)))) -200.0))) (.y (+ _returnvalue (* (`KismetMathLibrary.GetForwardVector` (`KismetMathLibrary.FindLookAtRotation` _returnvalue (`Actor.K2_GetActorLocation` (`GameplayStatics.GetPlayerCharacter` 0)))) -200.0))) (.z _returnvalue)) null
    (:`then`
      _)
    (:`OnSuccess`
      _)
    (:`OnFail`
      _))
  (set `CharacterMovementComponent.MaxWalkSpeed` 450.0 (`Character.CharacterMovement` _asbp_gnome))
  (`KismetSystemLibrary.Delay` 0.5)
  (add `/Game/MoTGF/Blueprints/Enemies/Gnome/BP_Gnome.OnReadyEnd` _asbp_gnome (delegate `ReadyEnd`))
  (`self.FinishExecute` true))

(event `ReadyEnd`)