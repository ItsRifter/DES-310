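; BP_Inventory is the player's weapon inventory, storing weapons in an array and handling switches between slots.
; It caches its owning BP_Player on BeginPlay, and AddWeapon starts or stops each weapon's use before appending it.
; ChangeItemFromSlot decrements the slot number into an array index, then, if that weapon is valid, stops the player's active weapon, activates the new one and prints its name.
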(event `self.ReceiveBeginPlay`
  (bind _asbp_player (cast `/Game/David/Blueprints/Player/BP_Player` (`self.GetOwner`)))
  (set `self.Player` _asbp_player))

(event `ChangeItemFromSlot`
  (params (ToSlot :type Integer))
  (bind _player (`self.Player`))
  (bind _activeweapon (`/Game/David/Blueprints/Player/BP_Player.ActiveWeapon` _player))
  (bind _output_get (set `self.CurrentSlot` ToSlot))
  (bind _result (`/Engine/EditorBlueprintResources/StandardMacros.DecrementInt` _output_get)
    (:`  `
      (bind _output (`|GetArrayItem` (`self.Weapons`) _result))
      (if (`KismetSystemLibrary.IsValid` _output)
        (if (`KismetSystemLibrary.IsValid` _activeweapon)
          (`/Game/David/Blueprints/Weapons/BP_WeaponBase.StopUsing` _activeweapon))
        (bind _output_get_2 (set `/Game/David/Blueprints/Player/BP_Player.ActiveWeapon` _output _player))
        (`/Game/David/Blueprints/Weapons/BP_WeaponBase.StartUsing` _output_get_2)
        (`KismetSystemLibrary.PrintString` (`KismetSystemLibrary.GetDisplayName` _output_get_2))))))

(event `AddWeapon`
  (params (ShouldStartUsing :type Boolean) (Weapon :type "/Game/David/Blueprints/Weapons/BP_WeaponBase Object Reference"))
  (if ShouldStartUsing
    (`/Game/David/Blueprints/Weapons/BP_WeaponBase.StartUsing` Weapon)
    (else
      (`/Game/David/Blueprints/Weapons/BP_WeaponBase.StopUsing` Weapon)))
  (`KismetArrayLibrary.Array_Add` (`self.Weapons`) Weapon))