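; Scythe weapon Blueprint that attacks by hitting an area rather than a single aimed target.
; DoAttack calls DoRadiusAttack with a zero target position and the weapon's Range as the radius.
; BeginPlay, OnObtain and construction only call the parent, and leftover HitTargets check and clear nodes are unwired.
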(event `self.ReceiveBeginPlay`
  (`parent.ReceiveBeginPlay`))

(event `self.OnObtain`
  (params (Player :type "/Game/MoTGF/Blueprints/Player/BP_Player Object Reference"))
  (`parent.OnObtain` Player))

(event `self.DoAttack`
  (`self.DoRadiusAttack` (0.0 0.0 0.0) (`self.Range`)))

(fn `UserConstructionScript`
  (`parent.UserConstructionScript`))