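; BP_Skill_Health is a skill Blueprint that raises the player's health when upgraded.
; CreateSkill only forwards the player to the parent implementation.
; Upgrade calls the parent, casts player character 0 to BP_Player, adds HealthUpPerLevel to its Health and prints the new value to screen.
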(event `self.CreateSkill`
  (params (Player :type "/Game/MoTGF/Blueprints/Player/BP_Player Object Reference"))
  (`parent.CreateSkill` Player))

(event `self.Upgrade`
  (`parent.Upgrade`)
  (bind _asbp_player (cast `/Game/MoTGF/Blueprints/Player/BP_Player` (`GameplayStatics.GetPlayerCharacter` 0)))
  (bind _output_get (set `/Game/MoTGF/Blueprints/Player/BP_Player.Health` (+ (`self.HealthUpPerLevel`) (`/Game/MoTGF/Blueprints/Player/BP_Player.Health` _asbp_player)) _asbp_player))
  (`KismetSystemLibrary.PrintString` (`KismetStringLibrary.Conv_DoubleToString` _output_get)))