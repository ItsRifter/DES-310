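; Room blueprint for procedural room generation, with north and south door triggers and a forest-clearing volume.
; When the player overlaps a door, it passes that door and the spawn locations to the matching parent door function.
; The ForestDestroyer volume passes any overlapping Forest actor to DestroyForest.
; An unconnected random room-spawn chain remains in the graph and never runs.
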(event `self.NorthDoor_0.OnComponentBeginOverlap`
  (params (OverlappedComponent :type "PrimitiveComponent Object Reference") (OtherActor :type "Actor Object Reference") (OtherComp :type "PrimitiveComponent Object Reference") (OtherBodyIndex :type Integer) (bFromSweep :type Boolean) (SweepResult :type "HitResult Structure (by ref)"))
  (cast `/Game/MoTGF/Blueprints/Player/BP_Player` OtherActor)
  (`parent.NorthDoor` (`self.NorthDoor_0`) (`self.SpawnLocations`)))

(event `self.SouthDoor_0.OnComponentBeginOverlap`
  (params (OverlappedComponent :type "PrimitiveComponent Object Reference") (OtherActor :type "Actor Object Reference") (OtherComp :type "PrimitiveComponent Object Reference") (OtherBodyIndex :type Integer) (bFromSweep :type Boolean) (SweepResult :type "HitResult Structure (by ref)"))
  (cast `/Game/MoTGF/Blueprints/Player/BP_Player` OtherActor)
  (`parent.SouthDoor` (`self.SouthDoor_0`) (`self.SpawnLocations`)))

(event `self.ForestDestroyer.OnComponentBeginOverlap`
  (params (OverlappedComponent :type "PrimitiveComponent Object Reference") (OtherActor :type "Actor Object Reference") (OtherComp :type "PrimitiveComponent Object Reference") (OtherBodyIndex :type Integer) (bFromSweep :type Boolean) (SweepResult :type "HitResult Structure (by ref)"))
  (bind _asforest (cast `/Game/MoTGF/Blueprints/RoomGeneration/Forest` OtherActor))
  (`self.DestroyForest` _asforest))

(fn `UserConstructionScript`)