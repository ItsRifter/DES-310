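; Room1 is a room actor that grows the level by spawning further copies of itself as the top-down character passes through its doors.
; North, East and South door overlaps spawn a new Room1 at a fixed grid offset in that direction and print the direction.
; A shared flag makes the first door overlap, presumably the entrance, spawn nothing.
; Later overlaps spawn every time, with no check for an existing neighbor.
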(event `self.NorthDoor.OnComponentBeginOverlap`
  (params (OverlappedComponent :type "PrimitiveComponent Object Reference") (OtherActor :type "Actor Object Reference") (OtherComp :type "PrimitiveComponent Object Reference") (OtherBodyIndex :type Integer) (bFromSweep :type Boolean) (SweepResult :type "HitResult Structure (by ref)"))
  (cast `/Game/TopDown/Blueprints/BP_TopDownCharacter` OtherActor)
  (if (`self.FirstDoorEntered`)
    (`|SpawnActorFromClass` "Room1_C" (`KismetMathLibrary.Conv_VectorToTransform` (+ (`self.K2_GetActorLocation`) (3500.0 0.0 0.0))) "Undefined" "MultiplyWithRoot" null null)
    (`KismetSystemLibrary.PrintString` "North")
    (else
      (set `self.FirstDoorEntered` true))))

(event `self.EastDoor.OnComponentBeginOverlap`
  (params (OverlappedComponent :type "PrimitiveComponent Object Reference") (OtherActor :type "Actor Object Reference") (OtherComp :type "PrimitiveComponent Object Reference") (OtherBodyIndex :type Integer) (bFromSweep :type Boolean) (SweepResult :type "HitResult Structure (by ref)"))
  (cast `/Game/TopDown/Blueprints/BP_TopDownCharacter` OtherActor)
  (if (`self.FirstDoorEntered`)
    (`|SpawnActorFromClass` "Room1_C" (`KismetMathLibrary.Conv_VectorToTransform` (+ (`self.K2_GetActorLocation`) (0.0 3500.0 0.0))) "Undefined" "MultiplyWithRoot" null null)
    (`KismetSystemLibrary.PrintString` "East")
    (else
      (set `self.FirstDoorEntered` true))))

(event `self.SouthDoor.OnComponentBeginOverlap`
  (params (OverlappedComponent :type "PrimitiveComponent Object Reference") (OtherActor :type "Actor Object Reference") (OtherComp :type "PrimitiveComponent Object Reference") (OtherBodyIndex :type Integer) (bFromSweep :type Boolean) (SweepResult :type "HitResult Structure (by ref)"))
  (cast `/Game/TopDown/Blueprints/BP_TopDownCharacter` OtherActor)
  (if (`self.FirstDoorEntered`)
    (`|SpawnActorFromClass` "Room1_C" (`KismetMathLibrary.Conv_VectorToTransform` (+ (`self.K2_GetActorLocation`) (-3500.0 0.0 0.0))) "Undefined" "MultiplyWithRoot" null null)
    (`KismetSystemLibrary.PrintString` "South")
    (else
      (set `self.FirstDoorEntered` true))))

(fn `UserConstructionScript`)