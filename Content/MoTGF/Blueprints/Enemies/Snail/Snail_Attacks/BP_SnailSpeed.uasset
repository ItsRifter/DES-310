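; Behavior tree task that sets the walk speed of snail enemies and snail bosses.
; It casts the controlled pawn through a chain: BP_Snail gets the task's MaxWalkSpeed variable, while the Average, Speedy and Tanky bosses get hardcoded speeds.
; It finishes successfully after setting the speed, but never calls FinishExecute if the pawn matches none of these classes.
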(event `self.ReceiveExecuteAI`
  (params (OwnerController :type "AIController Object Reference") (ControlledPawn :type "Pawn Object Reference"))
  (bind _asbp_snail (cast `/Game/MoTGF/Blueprints/Enemies/Snail/BP_Snail` ControlledPawn)
    (:`then`
      (set `CharacterMovementComponent.MaxWalkSpeed` (`self.Max Walk Speed`) (`Character.CharacterMovement` _asbp_snail))
      (`self.FinishExecute` true))
    (:`CastFailed`
      (bind _assnail_boss (cast `/Game/MoTGF/Blueprints/Enemies/Boss/SnailBossAverage` ControlledPawn)
        (:`then`
          (set `CharacterMovementComponent.MaxWalkSpeed` 400.0 (`Character.CharacterMovement` _assnail_boss))
          (`self.FinishExecute` true))
        (:`CastFailed`
          (bind _assnail_boss_speedy (cast `/Game/MoTGF/Blueprints/Enemies/Boss/SnailBossSpeedy` ControlledPawn)
            (:`then`
              (set `CharacterMovementComponent.MaxWalkSpeed` 600.0 (`Character.CharacterMovement` _assnail_boss_speedy))
              (`self.FinishExecute` true))
            (:`CastFailed`
              (bind _assnail_boss_tanky (cast `/Game/MoTGF/Blueprints/Enemies/Boss/SnailBossTanky` ControlledPawn))
              (set `CharacterMovementComponent.MaxWalkSpeed` 150.0 (`Character.CharacterMovement` _assnail_boss_tanky))
              (`self.FinishExecute` true))))))))