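; Door actor for room generation that can be locked or unlocked to block or open a passage.
; Lock shows the door mesh and enables its query and physics collision, while Unlock hides the mesh and disables collision, each updating the IsLocked flag.
; When the player overlaps the trigger box, the door calls DestroyForest, independent of its lock state.
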(event `Lock`
  (set `self.IsLocked` true)
  (`SceneComponent.SetVisibility` (`self.DoorMesh`) true true)
  (`PrimitiveComponent.SetCollisionEnabled` (`self.DoorMesh`) "QueryAndPhysics"))

(event `Unlock`
  (set `self.IsLocked` false)
  (`SceneComponent.SetVisibility` (`self.DoorMesh`) false true)
  (`PrimitiveComponent.SetCollisionEnabled` (`self.DoorMesh`) "NoCollision"))

(event `self.TriggerBox.OnComponentBeginOverlap`
  (params (OverlappedComponent :type "PrimitiveComponent Object Reference") (OtherActor :type "Actor Object Reference") (OtherComp :type "PrimitiveComponent Object Reference") (OtherBodyIndex :type Integer) (bFromSweep :type Boolean) (SweepResult :type "HitResult Structure (by ref)"))
  (cast `/Game/MoTGF/Blueprints/Player/BP_Player` OtherActor)
  (`self.DestroyForest` null))

(fn `UserConstructionScript`)