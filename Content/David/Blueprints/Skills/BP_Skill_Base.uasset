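; Base Blueprint for player skills, tracking a level and an upgrade cost and storing the owning Player on creation.
; Upgrade checks CanPurchaseLevel, which always returns true here, then increments the level and recalculates Cost as cost over level raised to PricePerLevelScale.
; RoundToDecimal floors using a Decimals × 10 factor rather than a power of ten, so two decimals yields 0.05 steps.
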(event `CreateSkill`
  (params (Player :type "/Game/David/Blueprints/Player/BP_Player Object Reference"))
  (set `self.Player` Player))

(event `Upgrade`
  (bind _curlevel (`self.CurLevel`))
  (bind _result (`self.CanPurchaseLevel`))
  (if _result
    (bind _result_2 (`/Engine/EditorBlueprintResources/StandardMacros.IncrementInt` _curlevel)
      (:`  `
        (set `self.CurLevel` _result_2)
        (bind _result_3 (`self.RoundToDecimal` (`KismetMathLibrary.MultiplyMultiply_FloatFloat` (/ (`self.Cost`) _curlevel) (`self.PricePerLevelScale`)) 2))
        (set `self.Cost` _result_3)))))

(fn `CanPurchaseLevel`
  (returns (Result :type Boolean))
  (return true))

(fn `RoundToDecimal`
  (params (Value :type "Float (double-precision)") (Decimals :type Integer))
  (returns (Result :type "Float (double-precision)"))
  (bind _returnvalue (* Decimals 10))
  (return (/ (`KismetMathLibrary.Conv_IntToDouble` (`KismetMathLibrary.FFloor` (* Value _returnvalue))) _returnvalue)))