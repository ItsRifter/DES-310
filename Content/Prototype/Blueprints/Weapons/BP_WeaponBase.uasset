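; Base weapon Blueprint that registers itself in the player's Weapons on pickup and toggles its root's visibility on use.
; DoAttack is an empty hook, alongside helpers for projectile, radius and arc attacks.
; Projectiles spawn with player rotation, and radius attacks sphere-trace a position without using the results.
; Arc attacks fan stepped sphere traces around player forward, collecting HitTargets; traces query WorldStatic with debug drawing, and no damage is applied.
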(event `StartUsing`
  (`SceneComponent.SetVisibility` (`self.DefaultSceneRoot`) true false))

(event `OnObtain`
  (params (Player :type "/Game/Prototype/Blueprints/Player/BP_Player Object Reference"))
  (bind _output_get (set `self.Player` Player))
  (`KismetArrayLibrary.Array_Add` (`/Game/Prototype/Blueprints/Player/BP_Player.Weapons` _output_get) self))

(event `StopUsing`
  (`SceneComponent.SetVisibility` (`self.DefaultSceneRoot`) false false))

(event `DoAttack`)

(event `DoProjectileAttack`
  (bind _returnvalue (`GameplayStatics.GetPlayerPawn` 0))
  ;[1 1 1] Projectile Attack
  (`|SpawnActorFromClass` (`self.Projectile`) (`KismetMathLibrary.MakeTransform` (0.0 0.0 0.0) (`self.K2_GetActorRotation` _returnvalue)) "AlwaysSpawn" "MultiplyWithRoot" _returnvalue null))

(event `DoArcAttack`
  (params (WepSteps :type Integer) (WepArcDist :type "Float (double-precision)") (WepRange :type "Float (double-precision)"))
  (bind _returnvalue (`GameplayStatics.GetPlayerCharacter` 0))
  (bind _returnvalue_2 (`self.K2_GetActorLocation` _returnvalue))
  ;[1 1 1] Arc / Swing Attack
  (set `self.Steps` WepSteps)
  (set `self.ArcDistance` WepArcDist)
  (set `self.Range` WepRange)
  (for _index (range 1 (+ (`self.Steps`) 1))
    (bind _outhits (`KismetSystemLibrary.SphereTraceMultiForObjects` :`Start` _returnvalue_2 :`End` (+ _returnvalue_2 (* (`KismetMathLibrary.GreaterGreater_VectorRotator` (`self.GetActorForwardVector` _returnvalue) (`KismetMathLibrary.MakeRotator` 0.0 0.0 (+ (* (`self.ArcDistance`) -0.5) (* _index (/ (`self.ArcDistance`) (`self.Steps`)))))) (`self.Range`))) :`Radius` 8.0 :`ObjectTypes` (`|MakeArray` "ObjectTypeQuery1" :!type "EObjectTypeQuery Enum") :`DrawDebugType` "ForDuration" :`DrawTime` 3.0))
    (for _array_element _outhits
      (`KismetArrayLibrary.Array_Add` (`self.HitTargets`) (`.HitActor` (`GameplayStatics.BreakHitResult` _array_element))))))

(event `DoRadiusAttack`
  (params (TargetPos :type "Vector Structure") (Radius :type "Float (double-precision)"))
  (bind _array (`|MakeArray` "ObjectTypeQuery1" :!type "EObjectTypeQuery Enum"))
  (bind _radius (`self.Radius`))
  (bind _position (`self.Position`))
  (bind _returnvalue (+ (* (`KismetMathLibrary.Vector_Down`) 32.0) (`self.K2_GetActorLocation` (`GameplayStatics.GetPlayerCharacter` 0))))
  ;[1 1 1] Circle / Radius Attack
  (set `self.Radius` Radius)
  (if (`KismetMathLibrary.Vector_IsZero` TargetPos)
    (`KismetSystemLibrary.SphereTraceMultiForObjects` :`Start` _returnvalue :`End` _returnvalue :`Radius` _radius :`ObjectTypes` _array :`DrawDebugType` "ForDuration" :`DrawTime` 3.0)
    (else
      (`KismetSystemLibrary.SphereTraceMultiForObjects` :`Start` _position :`End` _position :`Radius` _radius :`ObjectTypes` _array :`DrawDebugType` "ForDuration" :`DrawTime` 3.0))))

(fn `UserConstructionScript`)