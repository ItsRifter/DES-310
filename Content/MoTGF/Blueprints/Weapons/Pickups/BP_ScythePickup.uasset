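; BP_ScythePickup is a pickup actor that offers the scythe weapon to whatever overlaps its capsule.
; On BeginPlay it spawns a BP_Wep_Scythe and stores it in WeaponRef.
; Capsule overlap passes the other actor and that stored weapon to Pickup, whose logic is not defined here.
; An unconnected chain that adds a newly spawned scythe to the player's inventory and destroys the pickup never runs.
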(event `self.ReceiveBeginPlay`
  (bind _returnvalue (`|SpawnActorFromClass` "/Game/MoTGF/Blueprints/Weapons/Weapons/BP_Wep_Scythe.BP_Wep_Scythe_C" (`KismetMathLibrary.MakeTransform` (0.0 0.0 0.0)) "Undefined" "MultiplyWithRoot" null null))
  (set `self.WeaponRef` _returnvalue))

(event `self.Capsule.OnComponentBeginOverlap`
  (params (OverlappedComponent :type "PrimitiveComponent Object Reference") (OtherActor :type "Actor Object Reference") (OtherComp :type "PrimitiveComponent Object Reference") (OtherBodyIndex :type Integer) (bFromSweep :type Boolean) (SweepResult :type "HitResult Structure (by ref)"))
  (`self.Pickup` OtherActor (`self.WeaponRef`)))

(fn `UserConstructionScript`)