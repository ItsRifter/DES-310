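; Room9NS is a room Blueprint with north and south doors, used in room generation.
; It records both door transforms on BeginPlay, and when the player overlaps either door trigger it passes that door and the spawn locations to inherited door handlers.
; A one-shot collision box locks the doors on player entry, while the ForestDestroyer volume hands overlapping Forest actors to DestroyForest.
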(event `self.ReceiveBeginPlay`
  (`KismetArrayLibrary.Array_Add` (`self.DoorTransforms`) (`KismetMathLibrary.MakeTransform` (`SceneComponent.K2_GetComponentLocation` (`self.NorthDoor_0`)) (struct :`Yaw` 90.0)))
  (`KismetArrayLibrary.Array_Add` (`self.DoorTransforms`) (`KismetMathLibrary.MakeTransform` (`SceneComponent.K2_GetComponentLocation` (`self.SouthDoor_0`)) (struct :`Yaw` 90.0))))

(event `self.NorthDoor_0.OnComponentBeginOverlap`
  (params (OverlappedComponent :type "PrimitiveComponent Object Reference") (OtherActor :type "Actor Object Reference") (OtherComp :type "PrimitiveComponent Object Reference") (OtherBodyIndex :type Integer) (bFromSweep :type Boolean) (SweepResult :type "HitResult Structure (by ref)"))
  (cast `/Game/MoTGF/Blueprints/Player/BP_Player` OtherActor)
  (`parent.NorthDoor` (`self.NorthDoor_0`) (`self.SpawnLocations`)))

(event `self.SouthDoor_0.OnComponentBeginOverlap`
  (params (OverlappedComponent :type "PrimitiveComponent Object Reference") (OtherActor :type "Actor Object Reference") (OtherComp :type "PrimitiveComponent Object Reference") (OtherBodyIndex :type Integer) (bFromSweep :type Boolean) (SweepResult :type "HitResult Structure (by ref)"))
  (cast `/Game/MoTGF/Blueprints/Player/BP_Player` OtherActor)
  (`parent.SouthDoor` (`self.SouthDoor_0`) (`self.SpawnLocations`)))

(event `self.ForestDestroyer.OnComponentBeginOverlap`
  (params (OverlappedComponent :type "PrimitiveComponent Object Reference") (OtherActor :type "Actor Object Reference") (OtherComp :type "PrimitiveComponent Object Reference") (OtherBodyIndex :type Integer) (bFromSweep :type Boolean) (SweepResult :type "HitResult Structure (by ref)"))
  (bind _asforest (cast `/Game/MoTGF/Blueprints/RoomGeneration/Forest` OtherActor))
  (`self.DestroyForest` _asforest))

(event `self.DoorLockCollisionBox.OnComponentBeginOverlap`
  (params (OverlappedComponent :type "PrimitiveComponent Object Reference") (OtherActor :type "Actor Object Reference") (OtherComp :type "PrimitiveComponent Object Reference") (OtherBodyIndex :type Integer) (bFromSweep :type Boolean) (SweepResult :type "HitResult Structure (by ref)"))
  (cast `/Game/MoTGF/Blueprints/Player/BP_Player` OtherActor)
  (`ActorComponent.K2_DestroyComponent` (`self.DoorLockCollisionBox`))
  (`self.LockDoors` (`self.DoorTransforms`)))

(fn `UserConstructionScript`)