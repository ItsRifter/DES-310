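; BP_Wep_Dummy is a minimal child weapon Blueprint whose attack is a stab.
; DoAttack calls DoStabAttack with the weapon's Range and a zero attack radius.
; StartUsing is an empty override, while BeginPlay, OnObtain and the construction script only forward to the parent.
; Leftover HitTargets check and clear nodes are disconnected and never run.
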(event `self.StartUsing`)

(event `self.ReceiveBeginPlay`
  (`parent.ReceiveBeginPlay`))

(event `self.OnObtain`
  (params (Player :type "/Game/David/Blueprints/Player/BP_Player Object Reference"))
  (`parent.OnObtain` Player))

(event `self.DoAttack`
  (`self.DoStabAttack` (`self.Range`)))

(fn `UserConstructionScript`
  (`parent.UserConstructionScript`))