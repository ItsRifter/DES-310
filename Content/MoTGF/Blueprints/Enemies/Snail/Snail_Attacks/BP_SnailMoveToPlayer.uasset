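; Behavior Tree task that sends a snail enemy or snail boss toward the player character.
; It casts the controlled pawn to the regular, average, speedy or tanky snail class and runs AI MoveTo on player 0, with a wider acceptance radius for the tanky boss.
; Both move success and failure finish the task as successful.
; Any other pawn type leaves the task unfinished.
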(event `self.ReceiveExecuteAI`
  (params (OwnerController :type "AIController Object Reference") (ControlledPawn :type "Pawn Object Reference"))
  (bind _asbp_snail (cast `/Game/MoTGF/Blueprints/Enemies/Snail/BP_Snail` ControlledPawn)
    (:`then`
      (`|AIMoveTo` _asbp_snail (0.0 0.0 0.0) (`GameplayStatics.GetPlayerCharacter` 0) 100.0
        (:`OnSuccess`
          _)
        (:`OnFail`
          _))
      (`self.FinishExecute` true))
    (:`CastFailed`
      (bind _assnail_boss_average (cast `/Game/MoTGF/Blueprints/Enemies/Boss/SnailBossAverage` ControlledPawn)
        (:`then`
          (`|AIMoveTo` _assnail_boss_average (0.0 0.0 0.0) (`GameplayStatics.GetPlayerCharacter` 0) 100.0
            (:`OnSuccess`
              _)
            (:`OnFail`
              _))
          (`self.FinishExecute` true))
        (:`CastFailed`
          (bind _assnail_boss_speedy (cast `/Game/MoTGF/Blueprints/Enemies/Boss/SnailBossSpeedy` ControlledPawn)
            (:`then`
              (`|AIMoveTo` _assnail_boss_speedy (0.0 0.0 0.0) (`GameplayStatics.GetPlayerCharacter` 0) 100.0
                (:`OnSuccess`
                  _)
                (:`OnFail`
                  _))
              (`self.FinishExecute` true))
            (:`CastFailed`
              (bind _assnail_boss_tanky (cast `/Game/MoTGF/Blueprints/Enemies/Boss/SnailBossTanky` ControlledPawn))
              (`|AIMoveTo` _assnail_boss_tanky (0.0 0.0 0.0) (`GameplayStatics.GetPlayerCharacter` 0) 200.0
                (:`OnSuccess`
                  _)
                (:`OnFail`
                  _))
              (`self.FinishExecute` true))))))))