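; CentralRoom is the hub room for procedural room generation, spawning neighboring rooms as the player moves through it.
; When BP_Player overlaps the East or West door trigger, that trigger destroys itself and spawns a random class from the matching array at a fixed offset from the room.
; Separate East and West branch overlaps set LeftBranch on BP_TopDownGameMode to record the side taken.
; A south spawn path is left disconnected.
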(event `self.EastDoor.OnComponentBeginOverlap`
  (params (OverlappedComponent :type "PrimitiveComponent Object Reference") (OtherActor :type "Actor Object Reference") (OtherComp :type "PrimitiveComponent Object Reference") (OtherBodyIndex :type Integer) (bFromSweep :type Boolean) (SweepResult :type "HitResult Structure (by ref)"))
  (cast `/Game/MoTGF/Blueprints/Player/BP_Player` OtherActor)
  (`ActorComponent.K2_DestroyComponent` (`self.EastDoor`))
  (`|SpawnActorFromClass` (`|GetArrayItem` (`self.EastArray`) (`KismetMathLibrary.RandomIntegerInRange` 0 (- (`KismetArrayLibrary.Array_Length` (`self.EastArray`)) 1))) (`KismetMathLibrary.Conv_VectorToTransform` (+ (`self.K2_GetActorLocation`) (-250.0 2000.0 0.0))) "Undefined" "MultiplyWithRoot" null null))

(event `self.EastBranch.OnComponentBeginOverlap`
  (params (OverlappedComponent :type "PrimitiveComponent Object Reference") (OtherActor :type "Actor Object Reference") (OtherComp :type "PrimitiveComponent Object Reference") (OtherBodyIndex :type Integer) (bFromSweep :type Boolean) (SweepResult :type "HitResult Structure (by ref)"))
  (cast `/Game/MoTGF/Blueprints/Player/BP_Player` OtherActor)
  (bind _asbp_top_down_game_mode (cast `/Game/TopDown/Blueprints/BP_TopDownGameMode` (`GameplayStatics.GetGameMode`)))
  (set `/Game/TopDown/Blueprints/BP_TopDownGameMode.LeftBranch` false _asbp_top_down_game_mode))

(event `self.WestDoor.OnComponentBeginOverlap`
  (params (OverlappedComponent :type "PrimitiveComponent Object Reference") (OtherActor :type "Actor Object Reference") (OtherComp :type "PrimitiveComponent Object Reference") (OtherBodyIndex :type Integer) (bFromSweep :type Boolean) (SweepResult :type "HitResult Structure (by ref)"))
  (cast `/Game/MoTGF/Blueprints/Player/BP_Player` OtherActor)
  (`ActorComponent.K2_DestroyComponent` (`self.WestDoor`))
  (`|SpawnActorFromClass` (`|GetArrayItem` (`self.WestArray`) (`KismetMathLibrary.RandomIntegerInRange` 0 (- (`KismetArrayLibrary.Array_Length` (`self.WestArray`)) 1))) (`KismetMathLibrary.Conv_VectorToTransform` (+ (`self.K2_GetActorLocation`) (-250.0 -1500.0 0.0))) "Undefined" "MultiplyWithRoot" null null))

(event `self.WestBranch.OnComponentBeginOverlap`
  (params (OverlappedComponent :type "PrimitiveComponent Object Reference") (OtherActor :type "Actor Object Reference") (OtherComp :type "PrimitiveComponent Object Reference") (OtherBodyIndex :type Integer) (bFromSweep :type Boolean) (SweepResult :type "HitResult Structure (by ref)"))
  (cast `/Game/MoTGF/Blueprints/Player/BP_Player` OtherActor)
  (bind _asbp_top_down_game_mode (cast `/Game/TopDown/Blueprints/BP_TopDownGameMode` (`GameplayStatics.GetGameMode`)))
  (set `/Game/TopDown/Blueprints/BP_TopDownGameMode.LeftBranch` true _asbp_top_down_game_mode)
  (`KismetSystemLibrary.PrintText` "Hello"))

(fn `UserConstructionScript`)