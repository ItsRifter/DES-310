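; BP_Shop is an in-game shop that shows and hides a UI_Shop widget for the player.
; BeginPlay creates the widget hidden in the viewport, and opening or closing the shop just switches its visibility.
; ToggleShop works in both directions only while MoTGF_GameState reports a specific game status.
; Tick auto-closes an open shop once the player character stops overlapping ShopTrigger.
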(event `self.ReceiveTick`
  (params (DeltaSeconds :type "Float (single-precision)"))
  (bind _returnvalue (`PrimitiveComponent.IsOverlappingActor` (`self.Shop Trigger`) (`GameplayStatics.GetPlayerCharacter` 0)))
  (if (and (`self.IsShopOpen`) (not _returnvalue))
    (`self.CloseShop`)
    (elif _returnvalue
      _)))

(event `self.ReceiveBeginPlay`
  (bind _returnvalue (`|CreateWidget` "/Game/MoTGF/Blueprints/NewShop/UI_Shop.UI_Shop_C" (`GameplayStatics.GetPlayerController` 0)))
  (bind _output_get (set `self.WidgetUI` _returnvalue))
  (`UserWidget.AddToViewport` _returnvalue 0)
  (`Widget.SetVisibility` _output_get "Hidden"))

(event `ToggleShop`
  (bind _canbeopened (`self.CanOpen`))
  (if _canbeopened
    (if (`self.IsShopOpen`)
      (`self.CloseShop`)
      (else
        (`self.OpenShop`)))))

(event `OpenShop`
  (set `self.IsShopOpen` true)
  (`Widget.SetVisibility` (`self.WidgetUI`) "Visible"))

(event `CloseShop`
  (set `self.IsShopOpen` false)
  (`Widget.SetVisibility` (`self.WidgetUI`) "Hidden"))

(fn `CanOpen`
  (returns (CanBeOpened :type Boolean))
  (bind _asmo_tgf_game_state (cast `/Game/MoTGF/Blueprints/Gameplay/MoTGF_GameState` (`GameplayStatics.GetGameState`)))
  (bind _result (`/Game/MoTGF/Blueprints/Gameplay/MoTGF_GameState.IsAtGameStatus` _asmo_tgf_game_state "NewEnumerator1"))
  (return _result))

(fn `UserConstructionScript`)