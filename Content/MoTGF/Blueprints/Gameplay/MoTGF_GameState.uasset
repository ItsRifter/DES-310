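; Game state for MoTGF that runs the run loop through pre-run, timed active run and post-run phases, driven by bound dispatchers.
; Active runs count down a timer to end the run; post-run shows a stats screen and locks player movement.
; It also tracks enemies to clear doors, wipes rooms on reset and scales coin value by room count.
; MOTGF-prefixed debug functions force states, give weapons and set money.
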(event `SetGameState`
  (params (NewState :type "/Game/MoTGF/Blueprints/Gameplay/GameplayStates Enum" :default "NewEnumerator0"))
  ;[1 1 1] Sets game state to specific value
  (if (not (`|EnumEquality` NewState (`self.GameStatus`)))
    (set `self.GameStatus` NewState)
    (`self.UpdateGameStates`)))

(event `self.ReceiveTick`
  (params (DeltaSeconds :type "Float (single-precision)"))
  (switch `/Game/MoTGF/Blueprints/Gameplay/GameplayStates` (`self.GameStatus`)
    (:`NewEnumerator1`
      (`self.PreRunTick`))
    (:`NewEnumerator2`
      (`self.ActiveRunTick`))
    (:`NewEnumerator3`
      (`self.PostRunTick`))))

(event `NextGameState`
  ;[1 1 1] Updates gamestate to the next in run enum / Pre-Run to Post-Run and repeat
  (switch `/Game/MoTGF/Blueprints/Gameplay/GameplayStates` (`self.GameStatus`)
    (:`NewEnumerator0`
      (set `self.GameStatus` "NewEnumerator1"))
    (:`NewEnumerator1`
      (set `self.GameStatus` "NewEnumerator2"))
    (:`NewEnumerator2`
      (set `self.GameStatus` "NewEnumerator3"))
    (:`NewEnumerator3`
      (set `self.GameStatus` "NewEnumerator1")))
  (`self.UpdateGameStates`))

(event `PreRunTick`)

(event `ActiveRunTick`
  (bind _output_get (set `self.Timer` (- (`self.Timer`) (* (`GameplayStatics.GetWorldDeltaSeconds`) 1.0))))
  (if (<= _output_get 0.0)
    (`self.EndRun` "NewEnumerator1")))

(event `PostRunTick`)

(event `ResetPlayer`
  ;[1 1 1] Resets player
  (bind _asbp_player (cast `/Game/MoTGF/Blueprints/Player/BP_Player` (`GameplayStatics.GetPlayerPawn` 0)))
  (`/Game/MoTGF/Blueprints/Player/BP_Player.Respawn` _asbp_player)
  (bind _asbp_player_controller (cast `/Game/MoTGF/Blueprints/Player/BP_Player_Controller` (`GameplayStatics.GetPlayerController` 0)))
  (set `/Game/MoTGF/Blueprints/Player/BP_Player_Controller.RestrictMovement` false _asbp_player_controller))

(event `EnemyDeath`
  (bind _doorarray (`self.DoorArray`))
  (`/Engine/EditorBlueprintResources/StandardMacros.DecrementInt` (`self.EnemyCount`)
    (:`  `
      (if (<= (`self.EnemyCount`) 0)
        (for _array_element _doorarray
          (`self.K2_DestroyActor` _array_element))
        (`KismetArrayLibrary.Array_Clear` _doorarray)))))

(event `UpdateGameStates`
  ;[1 1 1] Update gameplay to reflect on new game state
  (switch `/Game/MoTGF/Blueprints/Gameplay/GameplayStates` (`self.GameStatus`)
    (:`NewEnumerator2`
      (set `self.Timer` 240.0))
    (:`NewEnumerator3`
      (`self.DoPostStatistics`))))

(event `DoPostStatistics`
  (bind _returnvalue (`GameplayStatics.GetPlayerController` 0))
  ;[1 1 1] Present post statistics to the player
  (bind _returnvalue_2 (`|CreateWidget` "/Game/MoTGF/Blueprints/UI/UI_PostScreen.UI_PostScreen_C" _returnvalue))
  (`UserWidget.AddToViewport` _returnvalue_2 0)
  (bind _asbp_player_controller (cast `/Game/MoTGF/Blueprints/Player/BP_Player_Controller` _returnvalue))
  (set `/Game/MoTGF/Blueprints/Player/BP_Player_Controller.RestrictMovement` true _asbp_player_controller))

(event `DoRoomReset`
  (bind _doorarray (`self.DoorArray`))
  (bind _enemyarray (`self.EnemyArray`))
  (bind _roomarray (`self.RoomArray`))
  (set `self.LeftDoorsEntered` 0)
  (set `self.RightDoorsEntered` 0)
  (set `self.EastCollision` true)
  (set `self.WestCollision` true)
  (for _array_element _roomarray
    (`self.K2_DestroyActor` _array_element))
  (`KismetArrayLibrary.Array_Clear` _roomarray)
  (for _array_element_2 _doorarray
    (`self.K2_DestroyActor` _array_element_2))
  (`KismetArrayLibrary.Array_Clear` _doorarray)
  (for _array_element_3 _enemyarray
    (if (`KismetSystemLibrary.IsValid` _array_element_3)
      (`self.K2_DestroyActor` _array_element_3)))
  (`KismetArrayLibrary.Array_Clear` _enemyarray)
  (set `self.EnemyCount` 0))

(event `self.ReceiveBeginPlay`
  (`self.SetGameState` "NewEnumerator0")
  (add `self.NewGame` (delegate `StartNewGame`))
  (add `self.BeginRun` (delegate `StartRun`))
  (add `self.EndRun` (delegate `ConcludeRun`))
  (add `self.FinishGame` (delegate `EndGame`))
  (add `self.ResetAllRooms` (delegate `ResetRun`))
  (`self.SetGameState` "NewEnumerator1"))

(event `StartNewGame`
  (`self.SetGameState` "NewEnumerator1"))

(event `ConcludeRun` :!signature `self.EndRun`
  (params (EndCondition :type "/Game/MoTGF/Blueprints/RoomGeneration/Enum_EndRunConditions Enum" :default "NewEnumerator0"))
  (`self.SetGameState` "NewEnumerator3"))

(event `EndGame`
  (`self.SetGameState` "NewEnumerator4"))

(event `ResetRun`
  (`self.DoRoomReset`)
  (`self.ResetPlayer`)
  (`self.SetGameState` "NewEnumerator1"))

(event `StartRun`
  (bind _result (`self.IsNotAtGameStatus` "NewEnumerator0"))
  (if _result
    (`self.SetGameState` "NewEnumerator2")))

(fn `DoCoinValueCalculations`
  (params (CoinValue :type Integer))
  (returns (CalcValue :type Integer))
  (bind _returnvalue (* (`|Copy` CoinValue) (/ (`KismetArrayLibrary.Array_Length` (`self.RoomArray`)) 3)))
  (if (< _returnvalue 1)
    (return CoinValue)
    (else
      (return _returnvalue))))

(fn `GetRunTimerToString`
  (returns (TimeString :type String))
  (return (`KismetStringLibrary.Conv_IntToString` (`KismetMathLibrary.Round` (`self.Timer`)))))

(fn `IsAtGameStatus`
  (params (Status :type "/Game/MoTGF/Blueprints/Gameplay/GameplayStates Enum" :default "NewEnumerator0"))
  (returns (Result :type Boolean))
  (return (`|EnumEquality` Status (`self.GameStatus`))))

(fn `IsNotAtGameStatus`
  (params (Status :type "/Game/MoTGF/Blueprints/Gameplay/GameplayStates Enum" :default "NewEnumerator0"))
  (returns (Result :type Boolean))
  (return (`|EnumInequality` Status (`self.GameStatus`))))

(fn `MOTGF_ForceGameState`
  (params (Gamestate :type "/Game/MoTGF/Blueprints/Gameplay/GameplayStates Enum" :default "NewEnumerator0"))
  (`self.SetGameState` Gamestate)
  (`self.UpdateGameStates`))

(fn `MOTGF_GiveWeapon`
  (params (WeaponName :type String))
  (switch `string` (`KismetStringLibrary.ToLower` WeaponName)
    (:`Default`
      (`KismetSystemLibrary.PrintString` "Couldn't spawn weapon - INVALID NAME" true true (struct :`R` 1.0 :`B` 0.043596 :`A` 1.0) 3.0))
    (:`spade`
      (bind _returnvalue (`|SpawnActorFromClass` "/Game/MoTGF/Blueprints/Weapons/Weapons/Bp_Wep_Pitchfork.Bp_Wep_Pitchfork_C" (`KismetMathLibrary.MakeTransform` (0.0 0.0 0.0)) "Undefined" "MultiplyWithRoot" null null))
      (bind _asbp_player (cast `/Game/MoTGF/Blueprints/Player/BP_Player` (`GameplayStatics.GetPlayerPawn` 0)))
      (`/Game/MoTGF/Blueprints/Player/BP_Inventory.AddWeapon` (`/Game/MoTGF/Blueprints/Player/BP_Player.Inventory` _asbp_player) false _returnvalue)
      (`KismetSystemLibrary.PrintString` "Gave 'Spade' weapon" true true (struct :`R` 0.341915 :`G` 1.0 :`A` 1.0) 3.0))
    (:`shovel`
      (bind _returnvalue_2 (`|SpawnActorFromClass` "/Game/MoTGF/Blueprints/Weapons/Weapons/BP_Wep_Shovel.BP_Wep_Shovel_C" (`KismetMathLibrary.MakeTransform` (0.0 0.0 0.0)) "Undefined" "MultiplyWithRoot" null null))
      (bind _asbp_player_2 (cast `/Game/MoTGF/Blueprints/Player/BP_Player` (`GameplayStatics.GetPlayerPawn` 0)))
      (`/Game/MoTGF/Blueprints/Player/BP_Inventory.AddWeapon` (`/Game/MoTGF/Blueprints/Player/BP_Player.Inventory` _asbp_player_2) false _returnvalue_2)
      (`KismetSystemLibrary.PrintString` "Gave 'Shovel' weapon" true true (struct :`R` 0.341915 :`G` 1.0 :`A` 1.0) 3.0))
    (:`scythe`
      (bind _returnvalue_3 (`|SpawnActorFromClass` "/Game/MoTGF/Blueprints/Weapons/Weapons/BP_Wep_Scythe.BP_Wep_Scythe_C" (`KismetMathLibrary.MakeTransform` (0.0 0.0 0.0)) "Undefined" "MultiplyWithRoot" null null))
      (bind _asbp_player_3 (cast `/Game/MoTGF/Blueprints/Player/BP_Player` (`GameplayStatics.GetPlayerPawn` 0)))
      (`/Game/MoTGF/Blueprints/Player/BP_Inventory.AddWeapon` (`/Game/MoTGF/Blueprints/Player/BP_Player.Inventory` _asbp_player_3) false _returnvalue_3)
      (`KismetSystemLibrary.PrintString` "Gave 'Scythe' weapon" true true (struct :`R` 0.341915 :`G` 1.0 :`A` 1.0) 3.0))
    (:`torcher`
      (bind _returnvalue_4 (`|SpawnActorFromClass` "/Game/MoTGF/Blueprints/Weapons/Weapons/BP_Wep_WeedTorcher.BP_Wep_WeedTorcher_C" (`KismetMathLibrary.MakeTransform` (0.0 0.0 0.0)) "Undefined" "MultiplyWithRoot" null null))
      (bind _asbp_player_4 (cast `/Game/MoTGF/Blueprints/Player/BP_Player` (`GameplayStatics.GetPlayerPawn` 0)))
      (`/Game/MoTGF/Blueprints/Player/BP_Inventory.AddWeapon` (`/Game/MoTGF/Blueprints/Player/BP_Player.Inventory` _asbp_player_4) false _returnvalue_4)
      (`KismetSystemLibrary.PrintString` "Gave 'Torcher' weapon" true true (struct :`R` 0.341915 :`G` 1.0 :`A` 1.0) 3.0))))

(fn `MOTGF_SetMoney`
  (params (Amount :type Integer))
  (bind _asbp_player (cast `/Game/MoTGF/Blueprints/Player/BP_Player` (`GameplayStatics.GetPlayerPawn` 0)))
  (set `/Game/MoTGF/Blueprints/Player/BP_Player.Money` Amount _asbp_player))

(fn `UserConstructionScript`)