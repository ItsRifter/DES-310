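; BP_Wep_Shovel is a melee shovel weapon built on a parent weapon Blueprint.
; Its attack event calls the inherited arc attack, passing its step count, arc distance and range.
; BeginPlay and construction only defer to the parent, and leftover hit-target checks are unconnected.
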(event `self.ReceiveBeginPlay`
  (`parent.ReceiveBeginPlay`))

(event `self.DoAttack`
  (`self.DoArcAttack` (`self.Steps`) (`self.ArcDistance`) (`self.Range`)))

(fn `UserConstructionScript`
  (`parent.UserConstructionScript`))