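; Forest Blueprint in the room generation folder, holding foliage components for trees, leaning trees, bushes and grass.
; On BeginPlay it creates one dynamic material instance from JoesTestMaterial and stores it in the Material variable.
; That shared instance replaces material slot 0 on the foliage components, so they all render from the same instance.
; Tick and the construction script are empty.
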(event `self.ReceiveBeginPlay`
  (bind _returnvalue (`KismetMaterialLibrary.CreateDynamicMaterialInstance` "/Game/MoTGF/Materials/JoesTestMaterial.JoesTestMaterial"))
  (bind _output_get (set `self.material` _returnvalue))
  (`PrimitiveComponent.SetMaterial` (`self.LeaningTree`) 0 _output_get)
  (`PrimitiveComponent.SetMaterial` (`self.LeaningTree1`) 0 _output_get)
  (`PrimitiveComponent.SetMaterial` (`self.Bush3`) 0 _output_get)
  (`PrimitiveComponent.SetMaterial` (`self.Bush4`) 0 _output_get)
  (`PrimitiveComponent.SetMaterial` (`self.Bush5`) 0 _output_get)
  (`PrimitiveComponent.SetMaterial` (`self.Bush`) 0 _output_get)
  (`PrimitiveComponent.SetMaterial` (`self.Grass2`) 0 _output_get)
  (`PrimitiveComponent.SetMaterial` (`self.Tree`) 0 _output_get)
  (`PrimitiveComponent.SetMaterial` (`self.Tree2`) 0 _output_get)
  (`PrimitiveComponent.SetMaterial` (`self.Tree3`) 0 _output_get)
  (`PrimitiveComponent.SetMaterial` (`self.Bush2`) 0 _output_get)
  (`PrimitiveComponent.SetMaterial` (`self.Grass10`) 0 _output_get)
  (`PrimitiveComponent.SetMaterial` (`self.Bush1`) 0 _output_get)
  (`PrimitiveComponent.SetMaterial` (`self.Tree1`) 0 _output_get)
  (`PrimitiveComponent.SetMaterial` (`self.Grass3`) 0 _output_get)
  (`PrimitiveComponent.SetMaterial` (`self.Grass4`) 0 _output_get)
  (`PrimitiveComponent.SetMaterial` (`self.Grass1`) 0 _output_get)
  (`PrimitiveComponent.SetMaterial` (`self.Grass6`) 0 _output_get)
  (`PrimitiveComponent.SetMaterial` (`self.Grass7`) 0 _output_get)
  (`PrimitiveComponent.SetMaterial` (`self.Grass9`) 0 _output_get)
  (`PrimitiveComponent.SetMaterial` (`self.Grass11`) 0 _output_get)
  (`PrimitiveComponent.SetMaterial` (`self.Grass8`) 0 _output_get)
  (`PrimitiveComponent.SetMaterial` (`self.Grass5`) 0 _output_get)
  (`PrimitiveComponent.SetMaterial` (`self.Grass`) 0 _output_get))

(fn `UserConstructionScript`)