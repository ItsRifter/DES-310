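; RoomManager procedurally builds the room layout at BeginPlay, starting from the placed Room_Central.
; GenerateRooms chains up to MaxRoomSpawn rooms using CreateAdjacentRoom's class and offset, following each room's first pathway left after removing the entry direction.
; OnRoomGenerated separately spawns a hidden adjacent room and increments doors.
; Door lock and enemy spawn events are empty, their logic left disconnected; alternate-path branching is only called from dead code.
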(event `LockDoors`
  (params (Doors :type "Array of /Game/MoTGF/Blueprints/NewRoomgeneration/Doorway Object Reference")))

(event `UnlockDoors`
  (params (Doors :type "Array of /Game/MoTGF/Blueprints/NewRoomgeneration/Doorway Object Reference")))

(event `SpawnEnemies`)

(event `self.ReceiveBeginPlay`
  (bind _returnvalue (`GameplayStatics.GetActorOfClass` "/Game/MoTGF/Blueprints/NewRoomgeneration/Rooms/Room_Central.Room_Central_C"))
  (bind _output_get (set `self.SpawnRoom` _returnvalue))
  (set `self.CurRoom` _output_get)
  (`self.GenerateRooms`))

(event `GenerateRooms`
  (set `self.RightBranchCreated` false)
  (set `self.LeftBranchCreated` false)
  (set `self.RoomsSpawned` 0)
  (while (< (`self.RoomsSpawned`) (`self.MaxRoomSpawn`))
    (`/Engine/EditorBlueprintResources/StandardMacros.IncrementInt` (`self.RoomsSpawned`)
      (:`  `
        (if (== (`GameplayStatics.GetObjectClass` (`self.CurRoom`)) "/Game/MoTGF/Blueprints/NewRoomgeneration/Rooms/Room_Central.Room_Central_C")
          (if (`self.LeftBranchCreated`)
            (bind (_roomclass _position) (`/Game/MoTGF/Blueprints/NewRoomgeneration/RoomFunctionLibrary.CreateAdjacentRoom` "NewEnumerator3"))
            (set `self.RightBranchCreated` true)
            (bind _returnvalue (`|SpawnActorFromClass` _roomclass (`KismetMathLibrary.MakeTransform` _position) "Undefined" "MultiplyWithRoot" null null))
            (bind _asroom_base (cast `/Game/MoTGF/Blueprints/NewRoomgeneration/Rooms/Room_Base` _returnvalue))
            (`/Game/MoTGF/Blueprints/NewRoomgeneration/Rooms/Room_Base.CreateRoom` _asroom_base "NewEnumerator3")
            (set `self.CurRoom` _asroom_base)
            (set `self.LastEntryDirection` "NewEnumerator3")
            (else
              (bind (_roomclass_2 _position_2) (`/Game/MoTGF/Blueprints/NewRoomgeneration/RoomFunctionLibrary.CreateAdjacentRoom` "NewEnumerator2"))
              (set `self.LeftBranchCreated` true)
              (bind _returnvalue_2 (`|SpawnActorFromClass` _roomclass_2 (`KismetMathLibrary.MakeTransform` _position_2) "Undefined" "MultiplyWithRoot" null null))
              (`/Game/MoTGF/Blueprints/NewRoomgeneration/Rooms/Room_Base.CreateRoom` _returnvalue_2 "NewEnumerator2")
              (set `self.CurRoom` _returnvalue_2)
              (set `self.LastEntryDirection` "NewEnumerator2")))
          (else
            (bind (_roomclass_3 _position_3) (`/Game/MoTGF/Blueprints/NewRoomgeneration/RoomFunctionLibrary.CreateAdjacentRoom` (`self.LastEntryDirection`)))
            (bind _returnvalue_3 (`|SpawnActorFromClass` _roomclass_3 (`KismetMathLibrary.MakeTransform` (+ (`self.K2_GetActorLocation` (`self.CurRoom`)) _position_3)) "Undefined" "MultiplyWithRoot" null null))
            (bind _output_get (set `self.CurRoom` _returnvalue_3))
            (`KismetArrayLibrary.Array_Add` (`self.AllRooms`) _output_get)
            (bind _output_get_2 (set `self.AvailablePathways` (`/Game/MoTGF/Blueprints/NewRoomgeneration/Rooms/Room_Base.Pathways` _output_get)))
            (`KismetArrayLibrary.Array_RemoveItem` _output_get_2 (`self.LastEntryDirection`))
            (bind _output_get_3 (set `self.LastEntryDirection` (`|GetArrayItem` _output_get_2)))
            (`KismetSystemLibrary.PrintString` (`|GetEnumeratorNameAsString` _output_get_3)))))))
  (if (and (`self.LeftBranchCreated`) (`self.RightBranchCreated`))
    _))

(event `GenerateAlternatePathRooms`
  (params (StartDirection :type "/Game/MoTGF/Blueprints/NewRoomgeneration/Enum_DirectionCompass Enum" :default "NewEnumerator4"))
  (bind (_roomclass _position) (`/Game/MoTGF/Blueprints/NewRoomgeneration/RoomFunctionLibrary.CreateAdjacentRoom` StartDirection))
  (`|SpawnActorFromClass` _roomclass (`KismetMathLibrary.MakeTransform` (+ (`self.K2_GetActorLocation` (`self.CurRoom`)) _position)) "Undefined" "MultiplyWithRoot" null null))

(fn `IsPlayer`
  (params (Actor :type "Actor Object Reference"))
  (returns (Result :type Boolean))
  (return (== (`GameplayStatics.GetObjectClass` Actor) null)))

(fn `On Room Generated`
  (params (Direction :type "/Game/MoTGF/Blueprints/NewRoomgeneration/Enum_DirectionCompass Enum" :default "NewEnumerator0") (RoomPos :type "Vector Structure"))
  (bind (_roomclass _position) (`/Game/MoTGF/Blueprints/NewRoomgeneration/RoomFunctionLibrary.CreateAdjacentRoom` Direction))
  (bind _returnvalue (`|SpawnActorFromClass` _roomclass (`KismetMathLibrary.MakeTransform` (+ _position RoomPos)) "Undefined" "MultiplyWithRoot" null null))
  (`/Game/MoTGF/Blueprints/NewRoomgeneration/Rooms/Room_Base.CreateRoom` _returnvalue Direction)
  (`SceneComponent.SetVisibility` (`/Game/MoTGF/Blueprints/NewRoomgeneration/Rooms/Room_Base.DefaultSceneRoot` _returnvalue) false true)
  (`/Game/MoTGF/Blueprints/NewRoomgeneration/RoomFunctionLibrary.IncrementDoors`))

(fn `UserConstructionScript`
  (bind _returnvalue (`AddComponent|NODE_AddBillboardComponent-1`))
  (`BillboardComponent.SetSprite` _returnvalue null))