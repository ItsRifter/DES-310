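; BP_Wall_Opacity is a component that hides walls blocking the camera's view of the player.
; Every Tick it line-traces the Camera channel from player camera to pawn, ignoring the pawn.
; A hit actor carrying this same component class is hidden entirely, with no opacity fade, and stored as LastHitWall.
; That wall is shown again only when a trace hits nothing, and only the last one stored is restored.
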(event `self.ReceiveTick`
  (params (DeltaSeconds :type "Float (single-precision)"))
  (bind _returnvalue (`GameplayStatics.GetPlayerPawn` 0))
  (bind _lasthitwall (`self.LastHitWall`))
  (bind (_outhit _returnvalue_2) (`KismetSystemLibrary.LineTraceSingle` (`PlayerCameraManager.GetCameraLocation` (`GameplayStatics.GetPlayerCameraManager` 0)) (`Actor.K2_GetActorLocation` _returnvalue) "TraceTypeQuery2" false (`|MakeArray` _returnvalue :!type "Actor Object Reference")))
  (if _returnvalue_2
    (bind (_bblockinghit _binitialoverlap _time _distance _location _impactpoint _normal _impactnormal _physmat _hitactor) (`GameplayStatics.BreakHitResult` _outhit))
    (if (`KismetSystemLibrary.IsValid` (`Actor.GetComponentByClass` _hitactor "BP_Wall_Opacity_C"))
      (`Actor.SetActorHiddenInGame` _hitactor true)
      (set `self.LastHitWall` _hitactor))
    (elif (`KismetSystemLibrary.IsValid` _lasthitwall)
      (`Actor.SetActorHiddenInGame` _lasthitwall false))))