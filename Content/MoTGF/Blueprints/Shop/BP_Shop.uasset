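; BP_Shop is an in-world shop with a fish character that reacts to the player and a toggleable shop UI.
; BeginPlay creates the UI_Shop widget, which is added to the viewport on first open and then shown or hidden, gated by game status.
; ShopTrigger overlaps play wave and leave montages with sounds, revealing the fish and spotlight on entry.
; Tick closes the shop when the player walks out of the trigger.
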(event `self.ReceiveTick`
  (params (DeltaSeconds :type "Float (single-precision)"))
  (bind _returnvalue (`PrimitiveComponent.IsOverlappingActor` (`self.Shop Trigger`) (`GameplayStatics.GetPlayerCharacter` 0)))
  (if (and (`self.IsShopOpen`) (not _returnvalue))
    (`self.CloseShop`)
    (elif _returnvalue
      _)))

(event `self.ReceiveBeginPlay`
  (bind _returnvalue (`|CreateWidget` "/Game/MoTGF/Blueprints/Shop/UI_Shop.UI_Shop_C" (`GameplayStatics.GetPlayerController` 0)))
  (set `self.WidgetUI` _returnvalue))

(event `ToggleShop`
  (bind _canbeopened (`self.CanOpen`))
  (if _canbeopened
    (if (`self.IsShopOpen`)
      (`self.CloseShop`)
      (else
        (`self.OpenShop`)))))

(event `OpenShop`
  (bind _widgetui (`self.WidgetUI`))
  (bind _asmo_tgf_game_state (cast `/Game/MoTGF/Blueprints/Gameplay/MoTGF_GameState` (`GameplayStatics.GetGameState`)))
  (bind _result (`/Game/MoTGF/Blueprints/Gameplay/MoTGF_GameState.IsAtGameStatus` _asmo_tgf_game_state "NewEnumerator1"))
  (if _result
    (set `self.IsShopOpen` true)
    (if (`self.IsShopCreated`)
      (`Widget.SetVisibility` _widgetui "Visible")
      (else
        (`UserWidget.AddToViewport` _widgetui 0)
        (set `self.IsShopCreated` true)))))

(event `CloseShop`
  (bind _asmo_tgf_game_state (cast `/Game/MoTGF/Blueprints/Gameplay/MoTGF_GameState` (`GameplayStatics.GetGameState`)))
  (bind _result (`/Game/MoTGF/Blueprints/Gameplay/MoTGF_GameState.IsAtGameStatus` _asmo_tgf_game_state "NewEnumerator1"))
  (if _result
    (set `self.IsShopOpen` false)
    (`Widget.SetVisibility` (`self.WidgetUI`) "Hidden")))

(event `self.Shop Trigger.OnComponentBeginOverlap`
  (params (OverlappedComponent :type "PrimitiveComponent Object Reference") (OtherActor :type "Actor Object Reference") (OtherComp :type "PrimitiveComponent Object Reference") (OtherBodyIndex :type Integer) (bFromSweep :type Boolean) (SweepResult :type "HitResult Structure (by ref)"))
  (bind _audio (`self.Audio`))
  (bind _asmo_tgf_game_state (cast `/Game/MoTGF/Blueprints/Gameplay/MoTGF_GameState` (`GameplayStatics.GetGameState`)))
  (bind _result (`/Game/MoTGF/Blueprints/Gameplay/MoTGF_GameState.IsNotAtGameStatus` _asmo_tgf_game_state "NewEnumerator2"))
  (if _result
    (cast `/Game/MoTGF/Blueprints/Player/BP_Player` OtherActor)
    (`SceneComponent.SetVisibility` (`self.FishSkeletalMesh`) true false)
    (`SceneComponent.SetVisibility` (`self.SpotLight`) true false)
    (`|PlayMontage` (`self.FishSkeletalMesh`) "/Game/MoTGF/Animations/Fish/FishWaveMontage.FishWaveMontage"
      (:`then`
        (`AudioComponent.SetSound` _audio "/Game/MoTGF/Sounds/shop_fish_entry.shop_fish_entry")
        (`AudioComponent.Play` _audio 0.0)))))

(event `self.Shop Trigger.OnComponentEndOverlap`
  (params (OverlappedComponent :type "PrimitiveComponent Object Reference") (OtherActor :type "Actor Object Reference") (OtherComp :type "PrimitiveComponent Object Reference") (OtherBodyIndex :type Integer))
  (bind _audio (`self.Audio`))
  (bind _asmo_tgf_game_state (cast `/Game/MoTGF/Blueprints/Gameplay/MoTGF_GameState` (`GameplayStatics.GetGameState`)))
  (bind _result (`/Game/MoTGF/Blueprints/Gameplay/MoTGF_GameState.IsNotAtGameStatus` _asmo_tgf_game_state "NewEnumerator2"))
  (if _result
    (cast `/Game/MoTGF/Blueprints/Player/BP_Player` OtherActor)
    (`|PlayMontage` (`self.FishSkeletalMesh`) "/Game/MoTGF/Animations/Fish/FishLeaveMontage.FishLeaveMontage"
      (:`then`
        (`AudioComponent.SetSound` _audio "/Game/MoTGF/Sounds/shop_fish_exit.shop_fish_exit")
        (`AudioComponent.Play` _audio 0.0)))))

(fn `CanOpen`
  (returns (CanBeOpened :type Boolean))
  (bind _asmo_tgf_game_state (cast `/Game/MoTGF/Blueprints/Gameplay/MoTGF_GameState` (`GameplayStatics.GetGameState`)))
  (bind _result (`/Game/MoTGF/Blueprints/Gameplay/MoTGF_GameState.IsAtGameStatus` _asmo_tgf_game_state "NewEnumerator1"))
  (return _result))

(fn `UserConstructionScript`)