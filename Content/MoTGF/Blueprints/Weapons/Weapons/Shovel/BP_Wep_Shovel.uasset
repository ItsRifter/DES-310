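; BP_Wep_Shovel is a melee shovel weapon built on a parent weapon Blueprint.
; On pickup it runs the parent obtain logic, then attaches to the ShovelSocket on the player's mesh, keeping relative transforms.
; Attacks pass a CanAttack check, then perform an arc attack and apply a cooldown through functions not defined in this file.
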(event `self.ReceiveBeginPlay`
  (`parent.ReceiveBeginPlay`))

(event `self.OnObtain`
  (params (Player :type "/Game/MoTGF/Blueprints/Player/BP_Player Object Reference"))
  (`parent.OnObtain` Player)
  (`self.K2_AttachToComponent` (`Character.Mesh` Player) "ShovelSocket" "KeepRelative" "KeepRelative" "KeepRelative"))

(event `self.DoAttack`
  (bind _canattack_ (`self.CanAttack`))
  (if _canattack_
    (`self.DoArcAttack`)
    (`self.ApplyCooldown`)))

(fn `UserConstructionScript`
  (`parent.UserConstructionScript`))