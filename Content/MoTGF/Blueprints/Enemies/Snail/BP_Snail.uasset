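; BP_Snail is a snail enemy with health, a widget health display and a shell form.
; On BeginPlay it fills the health UI, spawns its default controller and hides the shell.
; Attack, Ready and ShellForm events play montages and fire end callbacks, with the latter two swapping mesh visibility and sharing CallOnReadyEnd.
; Damage lowers health and updates the UI, while Tick destroys the actor once health runs out.
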(event `self.ReceiveBeginPlay`
  (bind _asbp_enemy_health_ui (cast `/Game/MoTGF/Blueprints/UI/BP_EnemyHealthUI` (`WidgetComponent.GetUserWidgetObject` (`self.Health`))))
  (bind _output_get (set `self.BP Health UI` _asbp_enemy_health_ui))
  (set `/Game/MoTGF/Blueprints/UI/BP_EnemyHealthUI.CurrentHealth` (`self.CurrentHealth`) _output_get)
  (set `/Game/MoTGF/Blueprints/UI/BP_EnemyHealthUI.MaxHealth` (`self.MaxHealth`) _output_get)
  (set `/Game/MoTGF/Blueprints/UI/BP_EnemyHealthUI.Enemy Type` (`self.EnemyName`) _output_get)
  (`self.SpawnDefaultController`)
  (`SceneComponent.SetVisibility` (`self.ShellForm`) false false))

(event `Attack`
  (`KismetSystemLibrary.PrintString` "ATTACK_S")
  (`|PlayMontage` (`self.Mesh`)
    (:`then`
      (`self.OnAttackEnd`))))

(event `Ready`
  (`KismetSystemLibrary.PrintString` "READY")
  (`SceneComponent.SetVisibility` (`self.Mesh`) true false)
  (`SceneComponent.SetVisibility` (`self.ShellForm`) false false)
  (`|PlayMontage` (`self.Mesh`)
    (:`then`
      (`self.OnReadyEnd`))))

(event `Shell Form`
  (`KismetSystemLibrary.PrintString` "SHELL")
  (`SceneComponent.SetVisibility` (`self.Mesh`) false false)
  (`SceneComponent.SetVisibility` (`self.ShellForm`) true false)
  (`|PlayMontage` (`self.Mesh`)
    (:`then`
      (`self.OnReadyEnd`))))

(event `self.ReceiveAnyDamage`
  (params (Damage :type "Float (single-precision)") (DamageType :type "DamageType Object Reference") (InstigatedBy :type "Controller Object Reference") (DamageCauser :type "Actor Object Reference"))
  (bind _output_get (set `self.CurrentHealth` (- (`self.CurrentHealth`) (* Damage 1.0))))
  (`/Game/MoTGF/Blueprints/UI/BP_EnemyHealthUI.Update Health` (`self.BP Health UI`) _output_get))

(event `self.ReceiveTick`
  (params (DeltaSeconds :type "Float (single-precision)"))
  (if (<= (`self.CurrentHealth`) 0)
    (`self.K2_DestroyActor`)))

(fn `UserConstructionScript`)