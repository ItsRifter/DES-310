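; BP_Player_Controller is the player controller for a mouse-cursor character, handling movement input and click-to-face.
; On BeginPlay it adds the Enhanced Input mapping context, caches BP_Player and shows the cursor.
; Unless restricted, IA_Movement moves the player relative to control rotation, re-facing the last clicked location while attacking.
; Left clicks, gated by EnableClick/DisableClick, trace under the cursor and send that hit location to the pawn through LookAtMessage.
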(event `self.ReceiveBeginPlay`
  (bind _returnvalue (subsystem `EnhancedInputLocalPlayerSubsystem`))
  (`/Engine/EditorBlueprintResources/StandardMacros.IsValid` _returnvalue
    (:`Is Valid`
      (`EnhancedInputSubsystemInterface.AddMappingContext` _returnvalue "/Game/MoTGF/Blueprints/Input/IMC_PlayerInput.IMC_PlayerInput" 0 (struct))
      (bind _asbp_player (cast `/Game/MoTGF/Blueprints/Player/BP_Player` (`GameplayStatics.GetPlayerCharacter` 0)))
      (set `self.PlayerRef` _asbp_player)
      (set `self.bShowMouseCursor` true))))

(event `EnhancedInput|/Game/MoTGF/Blueprints/Input/IA_Movement`
  (params (ActionValue :type "Vector2D Structure") (ElapsedSeconds :type "Float (double-precision)") (TriggeredSeconds :type "Float (double-precision)") (InputAction :type "InputAction Object Reference" :default "/Game/MoTGF/Blueprints/Input/IA_Movement.IA_Movement"))
  (bind (_returnvalue_roll _returnvalue_pitch _returnvalue_yaw) (`KismetMathLibrary.BreakRotator` (`self.GetControlRotation`)))
  (bind (_returnvalue_roll_2 _returnvalue_pitch_2 _returnvalue_yaw_2) (`KismetMathLibrary.BreakRotator` (`self.GetControlRotation`)))
  (:`Triggered`
    (if (not (`self.RestrictMovement`))
      (`Pawn.AddMovementInput` (`self.PlayerRef`) (* (`KismetMathLibrary.GetRightVector` (`KismetMathLibrary.MakeRotator` _returnvalue_roll_2 0.0 _returnvalue_yaw_2)) (`/Game/MoTGF/Blueprints/Player/BP_Player.Speed` (`self.PlayerRef`))) ActionValue_X false)
      (`Pawn.AddMovementInput` (`self.PlayerRef`) (* (`KismetMathLibrary.GetForwardVector` (`KismetMathLibrary.MakeRotator` 0.0 0.0 _returnvalue_yaw)) (`/Game/MoTGF/Blueprints/Player/BP_Player.Speed` (`self.PlayerRef`))) ActionValue_Y false)
      (if (`self.Attacking`)
        (message `/Game/MoTGF/Blueprints/Player/BP_LookAt.Look At` (`GameplayStatics.GetPlayerPawn` 0) (`self.MouseHitLocation`))))))

(event `Key|LeftMouseButton`
  (params (Key :type "Key Structure"))
  (:`Pressed`
    (if (`self.CheckLeftClicked`)
      (bind _output_get (set `self.MouseHitLocation` (`.Location` (`GameplayStatics.BreakHitResult` (`self.GetHitResultUnderCursorByChannel` "TraceTypeQuery1")))))
      (message `/Game/MoTGF/Blueprints/Player/BP_LookAt.Look At` (`GameplayStatics.GetPlayerPawn` 0) _output_get))))

(event `EnhancedInput|/Game/MoTGF/Blueprints/Input/IA_GamePad_Look`
  (params (ActionValue :type "Vector2D Structure") (ElapsedSeconds :type "Float (double-precision)") (TriggeredSeconds :type "Float (double-precision)") (InputAction :type "InputAction Object Reference" :default "/Game/MoTGF/Blueprints/Input/IA_GamePad_Look.IA_GamePad_Look")))

(fn `DisableClick`
  (set `self.CheckLeftClicked` false))

(fn `EnableClick`
  (set `self.CheckLeftClicked` true))

(fn `SetAttacking`
  (params (newAttacking :type Boolean))
  (set `self.Attacking` newAttacking))

(fn `UserConstructionScript`)