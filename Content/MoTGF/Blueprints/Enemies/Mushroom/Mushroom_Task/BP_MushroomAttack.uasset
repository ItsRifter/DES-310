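; Behavior tree task for the Mushroom enemy's area attack, which damages the player while the task runs.
; On execute it calls the mushroom's Attack and finishes successfully after a fixed delay; the bound attack-end handler is empty.
; Each tick, a sphere trace around the mushroom ignores Enemy-tagged actors and, on any pawn hit, damages player zero, throttled by a damage interval.
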(event `self.ReceiveExecuteAI`
  (params (OwnerController :type "AIController Object Reference") (ControlledPawn :type "Pawn Object Reference"))
  (bind _asbp_mushroom (cast `/Game/MoTGF/Blueprints/Enemies/Mushroom/BP_Mushroom` ControlledPawn))
  (`/Game/MoTGF/Blueprints/Enemies/Mushroom/BP_Mushroom.Attack` _asbp_mushroom)
  (add `/Game/MoTGF/Blueprints/Enemies/Mushroom/BP_Mushroom.OnAttackEnd` _asbp_mushroom (delegate `AttackEnd`))
  (`KismetSystemLibrary.Delay` 3.0)
  (`self.FinishExecute` true))

(event `AttackEnd`)

(event `self.ReceiveTickAI`
  (params (OwnerController :type "AIController Object Reference") (ControlledPawn :type "Pawn Object Reference") (DeltaSeconds :type "Float (single-precision)"))
  (bind _outactors (`GameplayStatics.GetAllActorsWithTag` "Enemy"))
  (bind _returnvalue (`Actor.K2_GetActorLocation` (stale `self.ReceiveExecuteAI` _asbp_mushroom)))
  (bind (_outhit _returnvalue_2) (`KismetSystemLibrary.SphereTraceSingleForObjects` _returnvalue _returnvalue 200.0 (`|MakeArray` "ObjectTypeQuery3" :!type "EObjectTypeQuery Enum") false _outactors "ForDuration" true (struct :`R` 1.0 :`A` 1.0) (struct :`G` 1.0 :`A` 1.0) 0.0))
  (if _returnvalue_2
    (if (<= (`self.TimeDamaged`) (- (`GameplayStatics.GetTimeSeconds`) (`self.DamageTickTime`)))
      (set `self.TimeDamaged` (`GameplayStatics.GetTimeSeconds`))
      (bind _asbp_player (cast `/Game/MoTGF/Blueprints/Player/BP_Player` (`GameplayStatics.GetPlayerPawn` 0)))
      (`GameplayStatics.ApplyDamage` _asbp_player 1.0))))